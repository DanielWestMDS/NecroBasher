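; Game mode for a round-based tower defense game that switches between combat and build phases.
; Tick polls HasRoundEnded, which advances the round and awards a skill point once no enemies remain.
; Between rounds it toggles the player's placement preview and countdown timer widget, resets the countdown once, and pauses for an unfinished build tutorial.
; Per-round lane warning logic is disconnected, leaving SetLaneWarning as an empty event.
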(event Custom|BetweenRounds
  (params (start%20time :type Float%20%28double-precision%29))
  (bind _asbp_first_person_character (Utilities|Casting|CastToBP_FirstPersonCharacter (Game|GetPlayerCharacter 0)))
  (if (Variables|/Game/FirstPerson/Blueprints/BP_FirstPersonCharacter.BP_FirstPersonCharacter_C|GetBuildTutoComp _asbp_first_person_character)
    _
    (else
      (Variables|/Game/FirstPerson/Blueprints/BP_FirstPersonCharacter.BP_FirstPersonCharacter_C|SetBuildTuto _asbp_first_person_character true)
      (Game|SetGamePaused true)))
  (if (not (Variables|Default|GetTimeSet))
    (Variables|/Game/UI/WB_Timer.WB_Timer_C|SetCountdown (Variables|Default|GetAs%20WB%20Timer) (Variables|Default|GetInitialTime))
    (Variables|Default|SetTimeSet true)))

(event Custom|SetLaneWarning)

(event EventTick
  (params (DeltaSeconds :type Float%20%28single-precision%29))
  (Utilities|FlowControl|Sequence
    (:then_0
      (Utilities|FlowControl|DoOnce false :!label _label
        (:Completed
          (CallFunction|SetLaneWarning))))
    (:then_1
      (bind _notinround (CallFunction|HasRoundEnded))
      (bind _asbp_first_person_character (Utilities|Casting|CastToBP_FirstPersonCharacter (Game|GetPlayerCharacter 0)))
      (bind _aswb_timer (Utilities|Casting|CastToWB_Timer (Variables|/Game/FirstPerson/Blueprints/BP_FirstPersonCharacter.BP_FirstPersonCharacter_C|GetTimerWidget _asbp_first_person_character)))
      (Variables|Default|SetAs%20WB%20Timer _aswb_timer)
      (if _notinround
        (if (> (Variables|/Game/FirstPerson/Blueprints/BP_FirstPersonCharacter.BP_FirstPersonCharacter_C|GetSelectedTower _asbp_first_person_character) 1)
          (Rendering|SetVisibility (Variables|/Game/FirstPerson/Blueprints/BP_FirstPersonCharacter.BP_FirstPersonCharacter_C|GetPlaceObject _asbp_first_person_character) true false))
        (CallFunction|BetweenRounds 0.0)
        (if (not (Variables|/Game/FirstPerson/Blueprints/BP_FirstPersonCharacter.BP_FirstPersonCharacter_C|GetbUpgradeOpen _asbp_first_person_character))
          (Widget|SetVisibility (Variables|Default|GetAs%20WB%20Timer) "Visible"))
        (else
          (Utilities|FlowControl|Sequence
            (:then_0
              (if (> (Variables|/Game/FirstPerson/Blueprints/BP_FirstPersonCharacter.BP_FirstPersonCharacter_C|GetSelectedTower _asbp_first_person_character) 1)
                (Rendering|SetVisibility (Variables|/Game/FirstPerson/Blueprints/BP_FirstPersonCharacter.BP_FirstPersonCharacter_C|GetPlaceObject _asbp_first_person_character) false false)
                (else
                  (Rendering|SetVisibility (Variables|/Game/FirstPerson/Blueprints/BP_FirstPersonCharacter.BP_FirstPersonCharacter_C|GetPlaceObject _asbp_first_person_character) false false))))
            (:then_1
              (Variables|Default|SetTimeSet false)
              (Widget|SetVisibility (Variables|Default|GetAs%20WB%20Timer) "Hidden"))))))
    (:then_2
      (if (not (Variables|Default|GetInRound))
        (goto _label Reset)))))

(fn ConstructionScript)

(fn HasRoundEnded
  (if (Variables|Default|GetInRound)
    (if (<= (Variables|Default|GetEnemiesAlive) 0)
      (Variables|Default|SetCurrentRound (+ (Variables|Default|GetCurrentRound) 1))
      (Variables|Default|SetSkillPoints (+ (Variables|Default|GetSkillPoints) 1))
      (Variables|Default|SetInRound false)
      (return true)
      (else
        (return false)))
    (else
      (return true))))