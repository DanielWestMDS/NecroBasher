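; Spline path actor that moves an array of placed actors continuously along its spline, following its position and rotation.
; A looping timeline, rate-scaled so TimelineLength sets the lap time, drives the distance along the spline.
; Each actor is offset by its index times OffsetBetweenActors and wraps once past the spline's end.
; The construction script applies the same spacing to lay the actors out from the spline start.
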(event Custom|PlayTimeline
  (bind _spline (Variables|Default|GetSpline))
  (bind _spline_2 (Variables|Default|GetSpline))
  (bind _returnvalue (Spline|GetSplineLength _spline))
  (bind _alpha (Timeline|Timeline PlayFromStart)
    (:Update
      (for (_array_element _array_index) (Variables|Default|GetActor)
        (bind _output_get (Variables|Default|SetDistanceAlongSpline (+ (Math|Float|Lerp 0.0 (Spline|GetSplineLength (Variables|Default|GetSpline)) _alpha) (* _array_index (Variables|Default|GetOffsetBetweenActors)))))
        (if (> _output_get _returnvalue)
          (Variables|Default|SetDistanceAlongSpline (- (Variables|Default|GetDistanceAlongSpline) _returnvalue)))
        (Transformation|SetActorLocationAndRotation _array_element (Spline|GetLocationatDistanceAlongSpline _spline_2 (Variables|Default|GetDistanceAlongSpline) "World") (Spline|GetRotationatDistanceAlongSpline _spline_2 (Variables|Default|GetDistanceAlongSpline) "World"))))
    (:Finished
      (CallFunction|PlayTimeline))))

(event EventBeginPlay
  ;[0.1094 0.1094 0.1094] Begin Play
  (Components|Timeline|SetPlayRate (Variables|Default|GetTimeline) (/ 1.0 (Variables|Default|GetTimelineLength)))
  (CallFunction|PlayTimeline))

(fn ConstructionScript
  (bind _spline (Variables|Default|GetSpline))
  (for (_array_element _array_index) (Variables|Default|GetActor)
    (Transformation|SetActorLocationAndRotation _array_element (Spline|GetLocationatDistanceAlongSpline _spline (* (Variables|Default|GetOffsetBetweenActors) _array_index) "World") (Spline|GetRotationatDistanceAlongSpline _spline (* (Variables|Default|GetOffsetBetweenActors) _array_index) "World"))))