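; Heavy enemy that travels along a chosen spline and periodically stops to turn toward the player and attack.
; Tick runs a countdown that triggers attack selection, which currently always picks the melee montage; the launching slam attack exists but is never selected.
; Rotation lerps between spline direction and player look-at, and health changes set a brief hurt flag.
; Death updates GameMode enemy count and currency, then ragdolls, explodes and destroys the actor.
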(event Custom|PickSpline
  ;[0.2024 0.2002 1] Spline Movement
  ;;[0.1094 0.1094 0.1094] Picks Spline to Move on
  (Variables|References|SetMovementSpline (Utilities|Array|Get(acopy) (Variables|References|GetSplineArrayReference) (Variables|SplineMovement|GetSplineValue))))

(event Custom|SlamAttack
  ;[1 0.2224 0.2483] Attacking stuff
  ;;[0.1094 0.1094 0.1094] Slam Attack
  (Variables|SplineMovement|SetMovingAlongSpline false)
  (CallFunction|RotateEnemy)
  (Utilities|FlowControl|Delay 2.0)
  (Variables|AttackSetting|SetIsSlamming true)
  (Development|PrintString "Slam Attack")
  (if (< (Transformation|GetDistanceTo (Variables|References|GetPlayerReference)) 5e+02)
    (Character|LaunchCharacter (Variables|References|GetPlayerReference) "0.000000,0.000000,1000.000000" false false))
  (Variables|AttackSetting|SetIsSlamAttack false)
  (Variables|AttackSetting|SetIsSlamming false)
  (Variables|SplineMovement|SetSplineTurningTick 0.0)
  (Variables|SplineMovement|SetMovingAlongSpline true))

(event Custom|SetMeleeBehaviourTimer
  ;[1 0.2224 0.2483] Attacking stuff
  ;;[0.1094 0.1094 0.1094] Timer for how often enemy attacks resets when 0
  (if (<= (Variables|AttackSetting|GetTimer) 0.0)
    (Development|PrintString "set timer")
    (Variables|AttackSetting|SetTimer 1e+01)
    (Variables|Default|SetbehaviourSelected false)
    (Variables|SplineMovement|SetSplineTurningTick 0.0)))

(event Custom|DecideMeleeAttack
  ;[1 0.2224 0.2483] Attacking stuff
  ;;[0.1094 0.1094 0.1094] Pick attack randomly
  (if (> (Math|Random|RandomFloat) 0.5)
    _
    (else
      _))
  (Variables|Default|SetisMeleeAttack true)
  (Development|PrintString "Melee Attack")
  (Variables|Default|SetbehaviourSelected true))

(event Custom|EnemyDeath
  (bind _gamemodereference (Variables|References|GetGameModeReference))
  ;[0 0 0] Handles Enemy Dying
  (Utilities|FlowControl|DoOnce false
    (:Completed
      ;;[0.1094 0.1094 0.1094] Decrement Global Enemy count
      (Variables|/Game/MiscBlueprints/BP_GameMode.BP_GameMode_C|SetEnemiesAlive _gamemodereference (- (Variables|/Game/MiscBlueprints/BP_GameMode.BP_GameMode_C|GetEnemiesAlive _gamemodereference) 1))
      ;;[0.1094 0.1094 0.1094] Give Currency To Player
      (Variables|/Game/MiscBlueprints/BP_GameMode.BP_GameMode_C|SetCurrency _gamemodereference (+ (Variables|/Game/MiscBlueprints/BP_GameMode.BP_GameMode_C|GetCurrency _gamemodereference) 100))
      (Variables|AttackSetting|SetcanAttack false)
      (Utilities|FlowControl|Delay 0.2)
      ;;[0.1094 0.1094 0.1094] DO NOT CHANGE THIS WHOLE GAME WILL BREAK IF YOU CHANGE THIS DO NOT CHANGE
      (Physics|SetSimulatePhysics (Variables|Character|GetMesh) true)
      (Utilities|FlowControl|Delay 3.0)
      (Niagara|SpawnSystematLocation "/Game/VFX_BEAM/VFX_Explosion.VFX_Explosion" (Transformation|GetSocketLocation (Variables|Character|GetMesh) "ChestSocket") "0, 0, 0" "1.200000,1.200000,1.200000")
      (Audio|PlaySoundatLocation "/Game/Sound/enemyDie.enemyDie" "0, 0, 0" "0, 0, 0" 1.0 1.0 0.0 0 0 0 0)
      (Utilities|FlowControl|Delay 0.1)
      (Actor|DestroyActor))))

(event Custom|RotateEnemy
  (bind _returnvalue (Transformation|GetActorLocation))
  (bind _playerreference (Variables|References|GetPlayerReference))
  (bind _movementspline (Variables|References|GetMovementSpline))
  (bind _distancealongspline (Variables|SplineMovement|GetDistanceAlongSpline))
  (bind _returnvalue_2 (Transformation|GetActorLocation _playerreference))
  (bind _spline (Variables|/Game/Enemies/BP_HeavyEnemySpline.BP_HeavyEnemySpline_C|GetSpline _movementspline))
  (bind _returnvalue_3 (Spline|GetRotationatDistanceAlongSpline _spline _distancealongspline "World"))
  (bind _returnvalue_4 (Math|Rotator|FindLookatRotation _returnvalue _returnvalue_2))
  ;[0.2024 0.2002 1] Spline Movement
  ;;[0.1844 0.1844 0.1844] Rotate Enemy towards player position
  (if (> (Variables|SplineMovement|GetSplineTurningTick) 1.0)
    _
    (else
      (Variables|SplineMovement|SetSplineTurningTick (+ (Utilities|Time|GetWorldDeltaSeconds) (Variables|SplineMovement|GetSplineTurningTick)))))
  (Transformation|SetActorRotation (Math|Rotator|MakeRotator (.roll (Math|Rotator|Lerp(Rotator) (Math|Rotator|MakeRotator (.roll _returnvalue_3) (.pitch _returnvalue_3) (.yaw _returnvalue_3)) (Math|Rotator|MakeRotator (.roll _returnvalue_4) (.pitch _returnvalue_4) (.yaw _returnvalue_4)) (Variables|SplineMovement|GetSplineTurningTick) true)) (.pitch (Math|Rotator|Lerp(Rotator) (Math|Rotator|MakeRotator (.roll _returnvalue_3) (.pitch _returnvalue_3) (.yaw _returnvalue_3)) (Math|Rotator|MakeRotator (.roll _returnvalue_4) (.pitch _returnvalue_4) (.yaw _returnvalue_4)) (Variables|SplineMovement|GetSplineTurningTick) true)) (.yaw (Math|Rotator|Lerp(Rotator) (Math|Rotator|MakeRotator (.roll _returnvalue_3) (.pitch _returnvalue_3) (.yaw _returnvalue_3)) (Math|Rotator|MakeRotator (.roll _returnvalue_4) (.pitch _returnvalue_4) (.yaw _returnvalue_4)) (Variables|SplineMovement|GetSplineTurningTick) true)))))

(event Custom|MovementAlongSpline
  (bind _movementspline (Variables|References|GetMovementSpline))
  (bind _spline (Variables|/Game/Enemies/BP_HeavyEnemySpline.BP_HeavyEnemySpline_C|GetSpline _movementspline))
  ;[0.2024 0.2002 1] Spline Movement
  ;;[0.1844 0.1844 0.1844] Movement for enemy along spline
  (Variables|SplineMovement|SetDistanceAlongSpline (+ (* (Utilities|Time|GetWorldDeltaSeconds) (Variables|SplineMovement|GetSplineSpeed)) (Variables|SplineMovement|GetDistanceAlongSpline)))
  (if (> (Variables|SplineMovement|GetSplineTurningTick) 1.0)
    _
    (else
      (Variables|SplineMovement|SetSplineTurningTick (+ (Utilities|Time|GetWorldDeltaSeconds) (Variables|SplineMovement|GetSplineTurningTick)))))
  (Transformation|SetActorLocation (Spline|GetLocationatDistanceAlongSpline _spline (Variables|SplineMovement|GetDistanceAlongSpline) "World") true false)
  (Transformation|SetActorRotation (Math|Rotator|Lerp(Rotator) (Math|Rotator|FindLookatRotation (Transformation|GetActorLocation) (Transformation|GetActorLocation (Variables|References|GetPlayerReference))) (Spline|GetRotationatDistanceAlongSpline _spline (Variables|SplineMovement|GetDistanceAlongSpline) "World") (Variables|SplineMovement|GetSplineTurningTick) true)))

(event Custom|MeleeAttack
  (bind _mesh (Variables|Character|GetMesh))
  (bind _returnvalue (Transformation|GetWorldLocation _mesh))
  ;[1 0.2224 0.2483] Attacking stuff
  ;;[0.1094 0.1094 0.1094] Melee Attack
  (Variables|SplineMovement|SetMovingAlongSpline false)
  (CallFunction|RotateEnemy)
  (Utilities|FlowControl|Delay 2.0)
  (Variables|AttackSetting|SetIsMeleeAttacking true)
  (Animation|Montage|PlayMontage (Variables|Character|GetMesh) "/Game/New_Enemy_Animations/Large_Enemy/AM_LargeEnemy.AM_LargeEnemy"
    (:then
      ;;[1 1 1] sound effects
      (Utilities|FlowControl|Delay 0.5)
      (Audio|PlaySoundatLocation "/Game/Sound/sword-slash-and-swing-185432.sword-slash-and-swing-185432" _returnvalue "0, 0, 0" 1.0 1.0 0.0 0 0 0 0)
      (Utilities|FlowControl|Delay 0.4)
      (Audio|PlaySoundatLocation "/Game/Sound/sword-slash-and-swing-185432.sword-slash-and-swing-185432" _returnvalue "0, 0, 0" 1.0 1.0 0.0 0 0 0 0))
    (:OnCompleted
      (Variables|AttackSetting|SetIsMeleeAttacking false)
      (Variables|AttackSetting|SetIsMeleeAttack false)
      (Variables|SplineMovement|SetSplineTurningTick 0.0)
      (Variables|SplineMovement|SetMovingAlongSpline true))))

(event EventBeginPlay
  ;[0.1662 1 0.2103] Comment
  ;;[0.1094 0.1094 0.1094] Begin play
  (Variables|SplineMovement|SetMovingAlongSpline true)
  (CallFunction|PickSpline)
  (bind _asbp_game_mode (Utilities|Casting|CastToBP_GameMode (Game|GetGameMode)))
  (Variables|References|SetGameModeReference _asbp_game_mode)
  (Variables|Default|SetHealth 1e+02)
  (bind _asbp_first_person_character (Utilities|Casting|CastToBP_FirstPersonCharacter (Game|GetPlayerCharacter 0)))
  (Variables|References|SetPlayerReference _asbp_first_person_character))

(event EventTick
  (params (DeltaSeconds :type Float%20%28single-precision%29))
  ;[0.3052 0.3052 0.3052] Main Event Tick
  (CallFunction|SetMeleeBehaviourTimer)
  (if (<= (Variables|Default|GetHealth) 0.0)
    (CallFunction|EnemyDeath)
    (else
      (Utilities|FlowControl|Sequence
        (:then_0
          ;;[0.1094 0.1094 0.1094] If no behaviour selected pick one, otherwise dont
          (if (Variables|Default|GetbehaviourSelected)
            _
            (else
              (CallFunction|DecideMeleeAttack)))
          (Variables|AttackSetting|SetTimer (- (Variables|AttackSetting|GetTimer) (Utilities|Time|GetWorldDeltaSeconds)))
          (Utilities|FlowControl|Sequence
            (:then_0
              ;;[0.1094 0.1094 0.1094] Based On selected behaviour
              (if (Variables|AttackSetting|GetIsSlamAttack)
                (CallFunction|SlamAttack)))
            (:then_1
              (if (Variables|AttackSetting|GetIsMeleeAttack)
                (CallFunction|MeleeAttack)))
            (:then_2
              (if (Variables|SplineMovement|GetMovingAlongSpline)
                (CallFunction|MovementAlongSpline)))))
        (:then_1
          ;;[1 1 1] for stun animation
          (if (not (== (Variables|Default|GetHealth) (Variables|Default|GetoldHealth)))
            (Variables|Default|SetoldHealth (Variables|Default|GetHealth))
            (Variables|Default|SetBeingHurt true)
            (Utilities|FlowControl|Delay 1.0)
            (Variables|Default|SetBeingHurt false)))))))

(fn ConstructionScript)

(fn DamagePlayer
  (bind _asbp_first_person_character (Utilities|Casting|CastToBP_FirstPersonCharacter (Game|GetPlayerCharacter 0)))
  (if (not (Variables|/Game/FirstPerson/Blueprints/BP_FirstPersonCharacter.BP_FirstPersonCharacter_C|GetbInvincible _asbp_first_person_character))
    (Variables|/Game/FirstPerson/Blueprints/BP_FirstPersonCharacter.BP_FirstPersonCharacter_C|SetLives _asbp_first_person_character (- (Variables|/Game/FirstPerson/Blueprints/BP_FirstPersonCharacter.BP_FirstPersonCharacter_C|GetLives _asbp_first_person_character) 1))))