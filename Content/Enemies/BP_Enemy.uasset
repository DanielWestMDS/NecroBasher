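; Enemy pawn that marches toward the main crystal, diverts to attack the player on sight, and destroys itself when Health runs out.
; Tick re-issues the move to the GameInstance's crystal location unless PawnSensing has seen the player, a flag that clears via a retriggerable delay.
; On reaching the player, a delayed sphere trace gates a distance-checked Health deduction.
; Crystal overlap only casts, with no effect.
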(event OnSeePawn(PawnSensing)
  (params (Pawn :type Pawn%20Object%20Reference))
  (Variables|Default|SetisSeeingPlayer true)
  (Utilities|FlowControl|Sequence
    (:then_0
      (CallFunction|MovetoPlayer))
    (:then_1
      (Utilities|FlowControl|RetriggerableDelay 0.6)
      (Variables|Default|SetisSeeingPlayer false))))

(event OnComponentBeginOverlap(CapsuleComponent)
  (params (OverlappedComponent :type Primitive%20Component%20Object%20Reference) (OtherActor :type Actor%20Object%20Reference) (OtherComp :type Primitive%20Component%20Object%20Reference) (OtherBodyIndex :type Integer) (bFromSweep :type Boolean) (SweepResult :type Hit%20Result%20Structure%20%28by%20ref%29))
  (Utilities|Casting|CastToBP_MainCrystal OtherActor))

(event Custom|MoveToPlayer
  (bind _mesh (Variables|Character|GetMesh))
  (bind _returnvalue (Transformation|GetWorldLocation _mesh))
  (Variables|Default|SetcanAttack true)
  (if (Variables|Default|GetisSeeingPlayer)
    (AI|AIMoveTo self "0, 0, 0" (Game|GetPlayerCharacter 0) 7e+01 false
      (:OnSuccess
        (if (Variables|Default|GetcanAttack)
          (Variables|Default|SetcanAttack false)
          (Utilities|FlowControl|Delay 1.5)
          (bind (_outhit _returnvalue_2) (Collision|SphereTraceByChannel _returnvalue (- _returnvalue "") 1.2e+02 "TraceTypeQuery1" false 0 "Persistent"))
          (if _returnvalue_2
            (Utilities|IsValid (Actor|GetComponentbyClass (.HitActor (Collision|BreakHitResult _outhit)) (Utilities|GetClass (.HitComponent (Collision|BreakHitResult _outhit))))
              (:Is%20Valid
                (CallFunction|AttackPlayer)
                (Variables|Default|SetcanAttack true)))))))
    (else
      (Variables|Default|SetisSeeingPlayer false)
      (Development|PrintString "see player false"))))

(event Custom|MoveToCrystal
  (if (not (Variables|Default|GetisSeeingPlayer))
    (bind _asbp_game_instance (Utilities|Casting|CastToBP_GameInstance (Game|GetGameInstance)))
    (AI|AIMoveTo self (Variables|/Game/FirstPerson/Blueprints/BP_GameInstance.BP_GameInstance_C|GetCrystalLocation _asbp_game_instance) 0 1.0 false)))

(event Custom|AttackPlayer
  ;[0.1177 0.1177 0.1177] AttackPlayer
  (bind _asbp_first_person_character (Utilities|Casting|CastToBP_FirstPersonCharacter (Game|GetPlayerCharacter 0)))
  (if (< (Transformation|GetDistanceTo _asbp_first_person_character) 2e+02)
    (Variables|/Game/FirstPerson/Blueprints/BP_FirstPersonCharacter.BP_FirstPersonCharacter_C|SetHealth _asbp_first_person_character (- (Variables|/Game/FirstPerson/Blueprints/BP_FirstPersonCharacter.BP_FirstPersonCharacter_C|GetHealth _asbp_first_person_character) 5e+01))
    (Development|PrintString "Attacks Player")))

(event Collision|EventActorBeginOverlap
  (params (OtherActor :type Actor%20Object%20Reference)))

(event EventTick
  (params (DeltaSeconds :type Float%20%28single-precision%29))
  (if (<= (Variables|Default|GetHealth) 0.0)
    (Actor|DestroyActor)
    (elif (not (Variables|Default|GetisSeeingPlayer))
      (Development|PrintString "Moving to crystal")
      (CallFunction|MovetoCrystal))))

(fn ConstructionScript)