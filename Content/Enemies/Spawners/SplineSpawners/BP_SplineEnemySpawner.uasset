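; Lane spawner that spawns attack, speed and flying enemies at its billboard over eight rounds, handing them ground or flying spline arrays.
; Tick calls InitializeRound for one-time per-round delay setup, then runs the current round's spawn event while InRound, after a global stagger delay.
; Per-type Delays pace spawning, gated by local round quotas and shared GameMode counts.
; Spawns decrement both counts, except round 1, which decrements only GameMode's.
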(event Custom|SpawnSpeedEnemy
  ;[0.1094 0.1094 0.1094] Spawn speed enemy at spawner location
  (bind _asbp_game_mode (Utilities|Casting|CastToBP_GameMode (Game|GetGameMode)))
  (Utilities|FlowControl|Delay (Variables|SpeedEnemySpawn|GetSpeedEnemySpawnDelay))
  (Game|SpawnActorfromClass "/Game/Enemies/BP_SpeedEnemy.BP_SpeedEnemy_C" (Math|Transform|MakeTransform (Transformation|GetWorldLocation (Variables|Default|GetBillboard)) "0, 0, 0" "1.000000,1.000000,1.000000") "Undefined" "MultiplyWithRoot" 0 (Variables|SplineArrays|GetGroundSplineArray) 0 2 0)
  (Variables|/Game/MiscBlueprints/BP_GameMode.BP_GameMode_C|SetNumSpeedEnemiesToSpawn _asbp_game_mode (- (Variables|/Game/MiscBlueprints/BP_GameMode.BP_GameMode_C|GetNumSpeedEnemiesToSpawn _asbp_game_mode) 1))
  (Utilities|FlowControl|Sequence
    (:then_0
      (if (== (Variables|/Game/MiscBlueprints/BP_GameMode.BP_GameMode_C|GetCurrentRound _asbp_game_mode) 1)
        _))
    (:then_1
      (if (== (Variables|/Game/MiscBlueprints/BP_GameMode.BP_GameMode_C|GetCurrentRound _asbp_game_mode) 2)
        (Variables|SpeedEnemySpawn|SetRound2SpeedEnemiesToSpawn (- (Variables|SpeedEnemySpawn|GetRound2SpeedEnemiesToSpawn) 1))))
    (:then_2
      (if (== (Variables|/Game/MiscBlueprints/BP_GameMode.BP_GameMode_C|GetCurrentRound _asbp_game_mode) 3)
        (Variables|SpeedEnemySpawn|SetRound3SpeedEnemiesToSpawn (- (Variables|SpeedEnemySpawn|GetRound3SpeedEnemiesToSpawn) 1))))
    (:then_3
      (if (== (Variables|/Game/MiscBlueprints/BP_GameMode.BP_GameMode_C|GetCurrentRound _asbp_game_mode) 4)
        (Variables|SpeedEnemySpawn|SetRound4SpeedEnemiesToSpawn (- (Variables|SpeedEnemySpawn|GetRound4SpeedEnemiesToSpawn) 1))))
    (:then_4
      (if (== (Variables|/Game/MiscBlueprints/BP_GameMode.BP_GameMode_C|GetCurrentRound _asbp_game_mode) 5)
        (Variables|SpeedEnemySpawn|SetRound5SpeedEnemiesToSpawn (- (Variables|SpeedEnemySpawn|GetRound5SpeedEnemiesToSpawn) 1))))
    (:then_5
      (if (== (Variables|/Game/MiscBlueprints/BP_GameMode.BP_GameMode_C|GetCurrentRound _asbp_game_mode) 6)
        (Variables|SpeedEnemySpawn|SetRound6SpeedEnemiesToSpawn (- (Variables|SpeedEnemySpawn|GetRound6SpeedEnemiesToSpawn) 1))))
    (:then_6
      (if (== (Variables|/Game/MiscBlueprints/BP_GameMode.BP_GameMode_C|GetCurrentRound _asbp_game_mode) 7)
        (Variables|SpeedEnemySpawn|SetRound7SpeedEnemiesToSpawn (- (Variables|SpeedEnemySpawn|GetRound7SpeedEnemiesToSpawn) 1))))
    (:then_7
      (if (== (Variables|/Game/MiscBlueprints/BP_GameMode.BP_GameMode_C|GetCurrentRound _asbp_game_mode) 8)
        (Variables|SpeedEnemySpawn|SetRound8SpeedEnemiesToSpawn (- (Variables|SpeedEnemySpawn|GetRound8SpeedEnemiesToSpawn) 1))))))

(event Custom|SpawnFlyingEnemy
  (bind _gamemodereference (Variables|References|GetGamemodeReference))
  (bind _currentround (Variables|/Game/MiscBlueprints/BP_GameMode.BP_GameMode_C|GetCurrentRound _gamemodereference))
  ;[0.1094 0.1094 0.1094] Spawn the Flying Enemy at spawner location
  (Utilities|FlowControl|Delay (Variables|FlyingEnemySpawn|GetFlyingEnemySpawnDelay))
  (Game|SpawnActorfromClass "/Game/Enemies/BP_FlyingEnemy.BP_FlyingEnemy_C" (Math|Transform|MakeTransform (Transformation|GetWorldLocation (Variables|Default|GetBillboard)) "0, 0, 0" "1.000000,1.000000,1.000000") "Undefined" "MultiplyWithRoot" 0 (Variables|SplineArrays|GetFlyingSplineArray) 3 0)
  (Variables|/Game/MiscBlueprints/BP_GameMode.BP_GameMode_C|SetNumFlyingEnemiesToSpawn _gamemodereference (- (Variables|/Game/MiscBlueprints/BP_GameMode.BP_GameMode_C|GetNumFlyingEnemiesToSpawn _gamemodereference) 1))
  (Utilities|FlowControl|Sequence
    (:then_0
      (if (== _currentround 1)
        _))
    (:then_1
      (if (== _currentround 2)
        (Variables|FlyingEnemySpawn|SetRound2FlyingEnemiesToSpawn (- (Variables|FlyingEnemySpawn|GetRound2FlyingEnemiesToSpawn) 1))))
    (:then_2
      (if (== _currentround 3)
        (Variables|FlyingEnemySpawn|SetRound3FlyingEnemiesToSpawn (- (Variables|FlyingEnemySpawn|GetRound3FlyingEnemiesToSpawn) 1))))
    (:then_3
      (if (== _currentround 4)
        (Variables|FlyingEnemySpawn|SetRound4FlyingEnemiesToSpawn (- (Variables|FlyingEnemySpawn|GetRound4FlyingEnemiesToSpawn) 1))))
    (:then_4
      (if (== _currentround 5)
        (Variables|FlyingEnemySpawn|SetRound5FlyingEnemiesToSpawn (- (Variables|FlyingEnemySpawn|GetRound5FlyingEnemiesToSpawn) 1))))
    (:then_5
      (if (== _currentround 6)
        (Variables|FlyingEnemySpawn|SetRound6FlyingEnemiesToSpawn (- (Variables|FlyingEnemySpawn|GetRound6FlyingEnemiesToSpawn) 1))))
    (:then_6
      (if (== _currentround 7)
        (Variables|FlyingEnemySpawn|SetRound7FlyingEnemiesToSpawn (- (Variables|FlyingEnemySpawn|GetRound7FlyingEnemiesToSpawn) 1))))
    (:then_7
      (if (== _currentround 8)
        (Variables|FlyingEnemySpawn|SetRound8FlyingEnemiesToSpawn (- (Variables|FlyingEnemySpawn|GetRound8FlyingEnemiesToSpawn) 1))))))

(event Custom|SpawnAttackEnemy
  (bind _gamemodereference (Variables|References|GetGamemodeReference))
  (bind _currentround (Variables|/Game/MiscBlueprints/BP_GameMode.BP_GameMode_C|GetCurrentRound _gamemodereference))
  ;[0.1094 0.1094 0.1094] Spawn the Attack Enemy at spawner location
  (Utilities|FlowControl|Delay (Variables|AttackEnemySpawn|GetAttackEnemySpawnDelay))
  (Game|SpawnActorfromClass "/Game/Enemies/BP_Enemy.BP_Enemy_C" (Math|Transform|MakeTransform (Transformation|GetWorldLocation (Variables|Default|GetBillboard)) "0, 0, 0" "1.000000,1.000000,1.000000") "Undefined" "MultiplyWithRoot" 0 (Variables|SplineArrays|GetGroundSplineArray) 0 2 0)
  (Development|PrintString "spawn enemy")
  (Variables|/Game/MiscBlueprints/BP_GameMode.BP_GameMode_C|SetNumAttackEnemiesToSpawn _gamemodereference (- (Variables|/Game/MiscBlueprints/BP_GameMode.BP_GameMode_C|GetNumAttackEnemiesToSpawn _gamemodereference) 1)) ; decrement num of attack enemies to be spawned
  (Utilities|FlowControl|Sequence
    (:then_0
      (if (== _currentround 1)
        _))
    (:then_1
      (if (== _currentround 2)
        (Variables|AttackEnemySpawn|SetRound2AttackEnemiesToSpawn (- (Variables|AttackEnemySpawn|GetRound2AttackEnemiesToSpawn) 1))))
    (:then_2
      (if (== _currentround 3)
        (Variables|AttackEnemySpawn|SetRound3AttackEnemiesToSpawn (- (Variables|AttackEnemySpawn|GetRound3AttackEnemiesToSpawn) 1))))
    (:then_3
      (if (== _currentround 4)
        (Variables|AttackEnemySpawn|SetRound4AttackEnemiesToSpawn (- (Variables|AttackEnemySpawn|GetRound4AttackEnemiesToSpawn) 1))))
    (:then_4
      (if (== _currentround 5)
        (Variables|AttackEnemySpawn|SetRound5AttackEnemiesToSpawn (- (Variables|AttackEnemySpawn|GetRound5AttackEnemiesToSpawn) 1))))
    (:then_5
      (if (== _currentround 6)
        (Variables|AttackEnemySpawn|SetRound6AttackEnemiesToSpawn (- (Variables|AttackEnemySpawn|GetRound6AttackEnemiesToSpawn) 1))))
    (:then_6
      (if (== _currentround 7)
        (Variables|AttackEnemySpawn|SetRound7AttackEnemiesToSpawn (- (Variables|AttackEnemySpawn|GetRound7AttackEnemiesToSpawn) 1))))
    (:then_7
      (if (== _currentround 8)
        (Variables|AttackEnemySpawn|SetRound8AttackEnemiesToSpawn (- (Variables|AttackEnemySpawn|GetRound8AttackEnemiesToSpawn) 1))))))

(event Custom|Round4EnemySpawn
  (bind _gamemodereference (Variables|References|GetGamemodeReference))
  ;[0.1094 0.1094 0.1094] Spawning Enemies in Round 4
  (Utilities|FlowControl|Sequence
    (:then_0
      (if (and (> (Variables|AttackEnemySpawn|GetRound4AttackEnemiesToSpawn) 0) (> (Variables|/Game/MiscBlueprints/BP_GameMode.BP_GameMode_C|GetNumAttackEnemiesToSpawn _gamemodereference) 0))
        (CallFunction|SpawnAttackEnemy)))
    (:then_1
      (if (and (> (Variables|/Game/MiscBlueprints/BP_GameMode.BP_GameMode_C|GetNumSpeedEnemiesToSpawn _gamemodereference) 0) (> (Variables|SpeedEnemySpawn|GetRound4SpeedEnemiesToSpawn) 0))
        (CallFunction|SpawnSpeedEnemy)))
    (:then_2
      (if (and (> (Variables|/Game/MiscBlueprints/BP_GameMode.BP_GameMode_C|GetNumFlyingEnemiesToSpawn _gamemodereference) 0) (> (Variables|FlyingEnemySpawn|GetRound4FlyingEnemiesToSpawn) 0))
        (CallFunction|SpawnFlyingEnemy)))))

(event Custom|Round5EnemySpawn
  (bind _gamemodereference (Variables|References|GetGamemodeReference))
  ;[0.1094 0.1094 0.1094] Spawning Enemies in Round 5
  (Utilities|FlowControl|Sequence
    (:then_0
      (if (and (> (Variables|AttackEnemySpawn|GetRound5AttackEnemiesToSpawn) 0) (> (Variables|/Game/MiscBlueprints/BP_GameMode.BP_GameMode_C|GetNumAttackEnemiesToSpawn _gamemodereference) 0))
        (CallFunction|SpawnAttackEnemy)))
    (:then_1
      (if (and (> (Variables|/Game/MiscBlueprints/BP_GameMode.BP_GameMode_C|GetNumSpeedEnemiesToSpawn _gamemodereference) 0) (> (Variables|SpeedEnemySpawn|GetRound5SpeedEnemiesToSpawn) 0))
        (CallFunction|SpawnSpeedEnemy)))
    (:then_2
      (if (and (> (Variables|/Game/MiscBlueprints/BP_GameMode.BP_GameMode_C|GetNumFlyingEnemiesToSpawn _gamemodereference) 0) (> (Variables|FlyingEnemySpawn|GetRound5FlyingEnemiesToSpawn) 0))
        (CallFunction|SpawnFlyingEnemy)))))

(event Custom|InitializeRound
  (bind _gamemodereference (Variables|References|GetGamemodeReference))
  ;[0.1083 0.1083 0.1083] Initialize each round with proper enemy amounts with cast to gamemode
  (if (== (Variables|/Game/MiscBlueprints/BP_GameMode.BP_GameMode_C|GetCurrentRound _gamemodereference) 1)
    (Utilities|FlowControl|DoOnce false
      (:Completed
        (Variables|/Game/MiscBlueprints/BP_GameMode.BP_GameMode_C|SetNumAttackEnemiesToSpawn _gamemodereference (Variables|/Game/MiscBlueprints/BP_GameMode.BP_GameMode_C|GetNumAttackEnemiesToSpawn _gamemodereference))
        (Variables|/Game/MiscBlueprints/BP_GameMode.BP_GameMode_C|SetNumSpeedEnemiesToSpawn _gamemodereference (Variables|/Game/MiscBlueprints/BP_GameMode.BP_GameMode_C|GetNumSpeedEnemiesToSpawn _gamemodereference))
        (Variables|/Game/MiscBlueprints/BP_GameMode.BP_GameMode_C|SetNumFlyingEnemiesToSpawn _gamemodereference (Variables|/Game/MiscBlueprints/BP_GameMode.BP_GameMode_C|GetNumFlyingEnemiesToSpawn _gamemodereference))
        (Variables|GlobalValuesForSpawner|SetGlobalSpawnDelay 2.0)
        (Variables|AttackEnemySpawn|SetAttackEnemySpawnDelay 2.0)
        (Variables|SpeedEnemySpawn|SetSpeedEnemySpawnDelay 2.0)
        (Variables|FlyingEnemySpawn|SetFlyingEnemySpawnDelay 3.0)
        (Variables|GlobalValuesForSpawner|SetHasGlobalDelayHappened false)))
    (elif (== (Variables|/Game/MiscBlueprints/BP_GameMode.BP_GameMode_C|GetCurrentRound _gamemodereference) 2)
      (Utilities|FlowControl|DoOnce false
        (:Completed
          (Variables|/Game/MiscBlueprints/BP_GameMode.BP_GameMode_C|SetNumAttackEnemiesToSpawn _gamemodereference (Variables|/Game/MiscBlueprints/BP_GameMode.BP_GameMode_C|GetNumAttackEnemiesToSpawn _gamemodereference))
          (Variables|/Game/MiscBlueprints/BP_GameMode.BP_GameMode_C|SetNumSpeedEnemiesToSpawn _gamemodereference (Variables|/Game/MiscBlueprints/BP_GameMode.BP_GameMode_C|GetNumSpeedEnemiesToSpawn _gamemodereference))
          (Variables|/Game/MiscBlueprints/BP_GameMode.BP_GameMode_C|SetNumFlyingEnemiesToSpawn _gamemodereference (Variables|/Game/MiscBlueprints/BP_GameMode.BP_GameMode_C|GetNumFlyingEnemiesToSpawn _gamemodereference))
          (Variables|GlobalValuesForSpawner|SetGlobalSpawnDelay 5.0)
          (Variables|AttackEnemySpawn|SetAttackEnemySpawnDelay 3.0)
          (Variables|SpeedEnemySpawn|SetSpeedEnemySpawnDelay 2.0)
          (Variables|FlyingEnemySpawn|SetFlyingEnemySpawnDelay 5.0)
          (Variables|GlobalValuesForSpawner|SetHasGlobalDelayHappened false)))
      (elif (== (Variables|/Game/MiscBlueprints/BP_GameMode.BP_GameMode_C|GetCurrentRound _gamemodereference) 3)
        (Utilities|FlowControl|DoOnce false
          (:Completed
            (Variables|/Game/MiscBlueprints/BP_GameMode.BP_GameMode_C|SetNumAttackEnemiesToSpawn _gamemodereference (Variables|/Game/MiscBlueprints/BP_GameMode.BP_GameMode_C|GetNumAttackEnemiesToSpawn _gamemodereference))
            (Variables|/Game/MiscBlueprints/BP_GameMode.BP_GameMode_C|SetNumSpeedEnemiesToSpawn _gamemodereference (Variables|/Game/MiscBlueprints/BP_GameMode.BP_GameMode_C|GetNumSpeedEnemiesToSpawn _gamemodereference))
            (Variables|/Game/MiscBlueprints/BP_GameMode.BP_GameMode_C|SetNumFlyingEnemiesToSpawn _gamemodereference (Variables|/Game/MiscBlueprints/BP_GameMode.BP_GameMode_C|GetNumFlyingEnemiesToSpawn _gamemodereference))
            (Variables|GlobalValuesForSpawner|SetGlobalSpawnDelay 3.0)
            (Variables|AttackEnemySpawn|SetAttackEnemySpawnDelay 3.0)
            (Variables|SpeedEnemySpawn|SetSpeedEnemySpawnDelay 2.0)
            (Variables|FlyingEnemySpawn|SetFlyingEnemySpawnDelay 5.0)
            (Variables|GlobalValuesForSpawner|SetHasGlobalDelayHappened false)))
        (elif (== (Variables|/Game/MiscBlueprints/BP_GameMode.BP_GameMode_C|GetCurrentRound _gamemodereference) 4)
          (Utilities|FlowControl|DoOnce false
            (:Completed
              (Variables|/Game/MiscBlueprints/BP_GameMode.BP_GameMode_C|SetNumAttackEnemiesToSpawn _gamemodereference (Variables|/Game/MiscBlueprints/BP_GameMode.BP_GameMode_C|GetNumAttackEnemiesToSpawn _gamemodereference))
              (Variables|/Game/MiscBlueprints/BP_GameMode.BP_GameMode_C|SetNumSpeedEnemiesToSpawn _gamemodereference (Variables|/Game/MiscBlueprints/BP_GameMode.BP_GameMode_C|GetNumSpeedEnemiesToSpawn _gamemodereference))
              (Variables|/Game/MiscBlueprints/BP_GameMode.BP_GameMode_C|SetNumFlyingEnemiesToSpawn _gamemodereference (Variables|/Game/MiscBlueprints/BP_GameMode.BP_GameMode_C|GetNumFlyingEnemiesToSpawn _gamemodereference))
              (Variables|GlobalValuesForSpawner|SetGlobalSpawnDelay 3.0)
              (Variables|AttackEnemySpawn|SetAttackEnemySpawnDelay 3.0)
              (Variables|SpeedEnemySpawn|SetSpeedEnemySpawnDelay 2.0)
              (Variables|FlyingEnemySpawn|SetFlyingEnemySpawnDelay 5.0)
              (Variables|GlobalValuesForSpawner|SetHasGlobalDelayHappened false)))
          (elif (== (Variables|/Game/MiscBlueprints/BP_GameMode.BP_GameMode_C|GetCurrentRound _gamemodereference) 5)
            (Utilities|FlowControl|DoOnce false
              (:Completed
                (Variables|/Game/MiscBlueprints/BP_GameMode.BP_GameMode_C|SetNumAttackEnemiesToSpawn _gamemodereference (Variables|/Game/MiscBlueprints/BP_GameMode.BP_GameMode_C|GetNumAttackEnemiesToSpawn _gamemodereference))
                (Variables|/Game/MiscBlueprints/BP_GameMode.BP_GameMode_C|SetNumSpeedEnemiesToSpawn _gamemodereference (Variables|/Game/MiscBlueprints/BP_GameMode.BP_GameMode_C|GetNumSpeedEnemiesToSpawn _gamemodereference))
                (Variables|/Game/MiscBlueprints/BP_GameMode.BP_GameMode_C|SetNumFlyingEnemiesToSpawn _gamemodereference (Variables|/Game/MiscBlueprints/BP_GameMode.BP_GameMode_C|GetNumFlyingEnemiesToSpawn _gamemodereference))
                (Variables|GlobalValuesForSpawner|SetGlobalSpawnDelay 3.0)
                (Variables|AttackEnemySpawn|SetAttackEnemySpawnDelay 3.0)
                (Variables|SpeedEnemySpawn|SetSpeedEnemySpawnDelay 2.0)
                (Variables|FlyingEnemySpawn|SetFlyingEnemySpawnDelay 5.0)
                (Variables|GlobalValuesForSpawner|SetHasGlobalDelayHappened false)))
            (elif (== (Variables|/Game/MiscBlueprints/BP_GameMode.BP_GameMode_C|GetCurrentRound _gamemodereference) 6)
              (Utilities|FlowControl|DoOnce false
                (:Completed
                  (Variables|/Game/MiscBlueprints/BP_GameMode.BP_GameMode_C|SetNumAttackEnemiesToSpawn _gamemodereference (Variables|/Game/MiscBlueprints/BP_GameMode.BP_GameMode_C|GetNumAttackEnemiesToSpawn _gamemodereference))
                  (Variables|/Game/MiscBlueprints/BP_GameMode.BP_GameMode_C|SetNumSpeedEnemiesToSpawn _gamemodereference (Variables|/Game/MiscBlueprints/BP_GameMode.BP_GameMode_C|GetNumSpeedEnemiesToSpawn _gamemodereference))
                  (Variables|/Game/MiscBlueprints/BP_GameMode.BP_GameMode_C|SetNumFlyingEnemiesToSpawn _gamemodereference (Variables|/Game/MiscBlueprints/BP_GameMode.BP_GameMode_C|GetNumFlyingEnemiesToSpawn _gamemodereference))
                  (Variables|GlobalValuesForSpawner|SetGlobalSpawnDelay 3.0)
                  (Variables|AttackEnemySpawn|SetAttackEnemySpawnDelay 3.0)
                  (Variables|SpeedEnemySpawn|SetSpeedEnemySpawnDelay 2.0)
                  (Variables|FlyingEnemySpawn|SetFlyingEnemySpawnDelay 5.0)
                  (Variables|GlobalValuesForSpawner|SetHasGlobalDelayHappened false)))
              (elif (== (Variables|/Game/MiscBlueprints/BP_GameMode.BP_GameMode_C|GetCurrentRound _gamemodereference) 7)
                (Utilities|FlowControl|DoOnce false
                  (:Completed
                    (Variables|/Game/MiscBlueprints/BP_GameMode.BP_GameMode_C|SetNumAttackEnemiesToSpawn _gamemodereference (Variables|/Game/MiscBlueprints/BP_GameMode.BP_GameMode_C|GetNumAttackEnemiesToSpawn _gamemodereference))
                    (Variables|/Game/MiscBlueprints/BP_GameMode.BP_GameMode_C|SetNumSpeedEnemiesToSpawn _gamemodereference (Variables|/Game/MiscBlueprints/BP_GameMode.BP_GameMode_C|GetNumSpeedEnemiesToSpawn _gamemodereference))
                    (Variables|/Game/MiscBlueprints/BP_GameMode.BP_GameMode_C|SetNumFlyingEnemiesToSpawn _gamemodereference (Variables|/Game/MiscBlueprints/BP_GameMode.BP_GameMode_C|GetNumFlyingEnemiesToSpawn _gamemodereference))
                    (Variables|GlobalValuesForSpawner|SetGlobalSpawnDelay 3.0)
                    (Variables|AttackEnemySpawn|SetAttackEnemySpawnDelay 3.0)
                    (Variables|SpeedEnemySpawn|SetSpeedEnemySpawnDelay 2.0)
                    (Variables|FlyingEnemySpawn|SetFlyingEnemySpawnDelay 5.0)
                    (Variables|GlobalValuesForSpawner|SetHasGlobalDelayHappened false)))
                (elif (== (Variables|/Game/MiscBlueprints/BP_GameMode.BP_GameMode_C|GetCurrentRound _gamemodereference) 8)
                  (Utilities|FlowControl|DoOnce false
                    (:Completed
                      (Variables|/Game/MiscBlueprints/BP_GameMode.BP_GameMode_C|SetNumAttackEnemiesToSpawn _gamemodereference (Variables|/Game/MiscBlueprints/BP_GameMode.BP_GameMode_C|GetNumAttackEnemiesToSpawn _gamemodereference))
                      (Variables|/Game/MiscBlueprints/BP_GameMode.BP_GameMode_C|SetNumSpeedEnemiesToSpawn _gamemodereference (Variables|/Game/MiscBlueprints/BP_GameMode.BP_GameMode_C|GetNumSpeedEnemiesToSpawn _gamemodereference))
                      (Variables|/Game/MiscBlueprints/BP_GameMode.BP_GameMode_C|SetNumFlyingEnemiesToSpawn _gamemodereference (Variables|/Game/MiscBlueprints/BP_GameMode.BP_GameMode_C|GetNumFlyingEnemiesToSpawn _gamemodereference))
                      (Variables|GlobalValuesForSpawner|SetGlobalSpawnDelay 3.0)
                      (Variables|AttackEnemySpawn|SetAttackEnemySpawnDelay 3.0)
                      (Variables|SpeedEnemySpawn|SetSpeedEnemySpawnDelay 2.0)
                      (Variables|FlyingEnemySpawn|SetFlyingEnemySpawnDelay 5.0)
                      (Variables|GlobalValuesForSpawner|SetHasGlobalDelayHappened false))))))))))))

(event Custom|RoundComplete
  ;[0.1094 0.1094 0.1094] When round completes initialize the next round
  (CallFunction|InitializeRound))

(event Custom|Round1EnemySpawn
  (bind _gamemodereference (Variables|References|GetGamemodeReference))
  ;[0.1094 0.1094 0.1094] Spawning Enemies in Round 1
  (Utilities|FlowControl|Sequence
    (:then_0
      (if (and (> (Variables|AttackEnemySpawn|GetRound1AttackEnemiesToSpawn) 0) (> (Variables|/Game/MiscBlueprints/BP_GameMode.BP_GameMode_C|GetNumAttackEnemiesToSpawn _gamemodereference) 0))
        (CallFunction|SpawnAttackEnemy)))
    (:then_1
      (if (and (> (Variables|/Game/MiscBlueprints/BP_GameMode.BP_GameMode_C|GetNumSpeedEnemiesToSpawn _gamemodereference) 0) (> (Variables|SpeedEnemySpawn|GetRound1SpeedEnemiesToSpawn) 0))
        (CallFunction|SpawnSpeedEnemy)))
    (:then_2
      (if (and (> (Variables|/Game/MiscBlueprints/BP_GameMode.BP_GameMode_C|GetNumFlyingEnemiesToSpawn _gamemodereference) 0) (> (Variables|FlyingEnemySpawn|GetRound1FlyingEnemiesToSpawn) 0))
        (CallFunction|SpawnFlyingEnemy)))))

(event Custom|Round7EnemySpawn
  (bind _gamemodereference (Variables|References|GetGamemodeReference))
  ;[0.1094 0.1094 0.1094] Spawning Enemies in Round 7
  (Utilities|FlowControl|Sequence
    (:then_0
      (if (and (> (Variables|AttackEnemySpawn|GetRound7AttackEnemiesToSpawn) 0) (> (Variables|/Game/MiscBlueprints/BP_GameMode.BP_GameMode_C|GetNumAttackEnemiesToSpawn _gamemodereference) 0))
        (CallFunction|SpawnAttackEnemy)))
    (:then_1
      (if (and (> (Variables|/Game/MiscBlueprints/BP_GameMode.BP_GameMode_C|GetNumSpeedEnemiesToSpawn _gamemodereference) 0) (> (Variables|SpeedEnemySpawn|GetRound7SpeedEnemiesToSpawn) 0))
        (CallFunction|SpawnSpeedEnemy)))
    (:then_2
      (if (and (> (Variables|/Game/MiscBlueprints/BP_GameMode.BP_GameMode_C|GetNumFlyingEnemiesToSpawn _gamemodereference) 0) (> (Variables|FlyingEnemySpawn|GetRound7FlyingEnemiesToSpawn) 0))
        (CallFunction|SpawnFlyingEnemy)))))

(event Custom|Round8EnemySpawn
  (bind _gamemodereference (Variables|References|GetGamemodeReference))
  ;[0.1094 0.1094 0.1094] Spawning Enemies in Round 8
  (Utilities|FlowControl|Sequence
    (:then_0
      (if (and (> (Variables|AttackEnemySpawn|GetRound8AttackEnemiesToSpawn) 0) (> (Variables|/Game/MiscBlueprints/BP_GameMode.BP_GameMode_C|GetNumAttackEnemiesToSpawn _gamemodereference) 0))
        (CallFunction|SpawnAttackEnemy)))
    (:then_1
      (if (and (> (Variables|/Game/MiscBlueprints/BP_GameMode.BP_GameMode_C|GetNumSpeedEnemiesToSpawn _gamemodereference) 0) (> (Variables|SpeedEnemySpawn|GetRound8SpeedEnemiesToSpawn) 0))
        (CallFunction|SpawnSpeedEnemy)))
    (:then_2
      (if (and (> (Variables|/Game/MiscBlueprints/BP_GameMode.BP_GameMode_C|GetNumFlyingEnemiesToSpawn _gamemodereference) 0) (> (Variables|FlyingEnemySpawn|GetRound8FlyingEnemiesToSpawn) 0))
        (CallFunction|SpawnFlyingEnemy)))))

(event Custom|Round6EnemySpawn
  (bind _gamemodereference (Variables|References|GetGamemodeReference))
  ;[0.1094 0.1094 0.1094] Spawning Enemies in Round 6
  (Utilities|FlowControl|Sequence
    (:then_0
      (if (and (> (Variables|AttackEnemySpawn|GetRound6AttackEnemiesToSpawn) 0) (> (Variables|/Game/MiscBlueprints/BP_GameMode.BP_GameMode_C|GetNumAttackEnemiesToSpawn _gamemodereference) 0))
        (CallFunction|SpawnAttackEnemy)))
    (:then_1
      (if (and (> (Variables|/Game/MiscBlueprints/BP_GameMode.BP_GameMode_C|GetNumSpeedEnemiesToSpawn _gamemodereference) 0) (> (Variables|SpeedEnemySpawn|GetRound6SpeedEnemiesToSpawn) 0))
        (CallFunction|SpawnSpeedEnemy)))
    (:then_2
      (if (and (> (Variables|/Game/MiscBlueprints/BP_GameMode.BP_GameMode_C|GetNumFlyingEnemiesToSpawn _gamemodereference) 0) (> (Variables|FlyingEnemySpawn|GetRound6FlyingEnemiesToSpawn) 0))
        (CallFunction|SpawnFlyingEnemy)))))

(event Custom|Round2EnemySpawn
  (bind _gamemodereference (Variables|References|GetGamemodeReference))
  ;[0.1094 0.1094 0.1094] Spawning Enemies in Round 2
  (Utilities|FlowControl|Sequence
    (:then_0
      (if (and (> (Variables|AttackEnemySpawn|GetRound2AttackEnemiesToSpawn) 0) (> (Variables|/Game/MiscBlueprints/BP_GameMode.BP_GameMode_C|GetNumAttackEnemiesToSpawn _gamemodereference) 0))
        (CallFunction|SpawnAttackEnemy)))
    (:then_1
      (if (and (> (Variables|/Game/MiscBlueprints/BP_GameMode.BP_GameMode_C|GetNumSpeedEnemiesToSpawn _gamemodereference) 0) (> (Variables|SpeedEnemySpawn|GetRound2SpeedEnemiesToSpawn) 0))
        (CallFunction|SpawnSpeedEnemy)))
    (:then_2
      (if (and (> (Variables|/Game/MiscBlueprints/BP_GameMode.BP_GameMode_C|GetNumFlyingEnemiesToSpawn _gamemodereference) 0) (> (Variables|FlyingEnemySpawn|GetRound2FlyingEnemiesToSpawn) 0))
        (CallFunction|SpawnFlyingEnemy)))))

(event Custom|Round3EnemySpawn
  (bind _gamemodereference (Variables|References|GetGamemodeReference))
  ;[0.1094 0.1094 0.1094] Spawning Enemies in Round 3
  (Utilities|FlowControl|Sequence
    (:then_0
      (if (and (> (Variables|AttackEnemySpawn|GetRound3AttackEnemiesToSpawn) 0) (> (Variables|/Game/MiscBlueprints/BP_GameMode.BP_GameMode_C|GetNumAttackEnemiesToSpawn _gamemodereference) 0))
        (CallFunction|SpawnAttackEnemy)))
    (:then_1
      (if (and (> (Variables|/Game/MiscBlueprints/BP_GameMode.BP_GameMode_C|GetNumSpeedEnemiesToSpawn _gamemodereference) 0) (> (Variables|SpeedEnemySpawn|GetRound3SpeedEnemiesToSpawn) 0))
        (CallFunction|SpawnSpeedEnemy)))
    (:then_2
      (if (and (> (Variables|/Game/MiscBlueprints/BP_GameMode.BP_GameMode_C|GetNumFlyingEnemiesToSpawn _gamemodereference) 0) (> (Variables|FlyingEnemySpawn|GetRound3FlyingEnemiesToSpawn) 0))
        (CallFunction|SpawnFlyingEnemy)))))

(event EventBeginPlay
  ;[0.1094 0.1094 0.1094] Begin play to get gamemode reference to avoid multiple casts
  (bind _asbp_game_mode (Utilities|Casting|CastToBP_GameMode (Game|GetGameMode)))
  (Variables|References|SetGamemodeReference _asbp_game_mode)
  (for _array_element (Variables|SplineArrays|GetGroundSplineArray)
    (Development|PrintString (Utilities|GetDisplayName _array_element))))

(event EventTick
  (params (DeltaSeconds :type Float%20%28single-precision%29))
  (bind _gamemodereference (Variables|References|GetGamemodeReference))
  (CallFunction|InitializeRound)
  ;[0.1094 0.1094 0.1094] If player is in round spawn enemies
  (if (Variables|/Game/MiscBlueprints/BP_GameMode.BP_GameMode_C|GetInRound _gamemodereference)
    (if (Variables|GlobalValuesForSpawner|GetHasGlobalDelayHappened)
      _
      (else
        (Utilities|FlowControl|Delay (Variables|GlobalValuesForSpawner|GetGlobalSpawnDelay)) ; Spawn delay on spawner if you wanted to \nsay stagger certain lanes
        (Variables|GlobalValuesForSpawner|SetHasGlobalDelayHappened true)))
    ;[0.1094 0.1094 0.1094] Spawn enemies based on round
    (Utilities|FlowControl|Sequence
      (:then_0
        (if (== (Variables|/Game/MiscBlueprints/BP_GameMode.BP_GameMode_C|GetCurrentRound _gamemodereference) 1)
          (CallFunction|Round1EnemySpawn)))
      (:then_1
        (if (== (Variables|/Game/MiscBlueprints/BP_GameMode.BP_GameMode_C|GetCurrentRound _gamemodereference) 2)
          (CallFunction|Round2EnemySpawn)))
      (:then_2
        (if (== (Variables|/Game/MiscBlueprints/BP_GameMode.BP_GameMode_C|GetCurrentRound _gamemodereference) 3)
          (CallFunction|Round3EnemySpawn)))
      (:then_3
        (if (== (Variables|/Game/MiscBlueprints/BP_GameMode.BP_GameMode_C|GetCurrentRound _gamemodereference) 4)
          (CallFunction|Round4EnemySpawn)))
      (:then_4
        (if (== (Variables|/Game/MiscBlueprints/BP_GameMode.BP_GameMode_C|GetCurrentRound _gamemodereference) 5)
          (CallFunction|Round5EnemySpawn)))
      (:then_5
        (if (== (Variables|/Game/MiscBlueprints/BP_GameMode.BP_GameMode_C|GetCurrentRound _gamemodereference) 6)
          (CallFunction|Round6EnemySpawn)))
      (:then_6
        (if (== (Variables|/Game/MiscBlueprints/BP_GameMode.BP_GameMode_C|GetCurrentRound _gamemodereference) 7)
          (CallFunction|Round7EnemySpawn)))
      (:then_7
        (if (== (Variables|/Game/MiscBlueprints/BP_GameMode.BP_GameMode_C|GetCurrentRound _gamemodereference) 8)
          (CallFunction|Round8EnemySpawn))))
    (else
      (CallFunction|RoundComplete))))

(fn ConstructionScript)