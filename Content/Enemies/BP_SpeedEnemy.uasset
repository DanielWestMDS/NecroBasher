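; BP_SpeedEnemy is an enemy that loops a movement animation and heads for the crystal location stored in BP_GameInstance.
; Tick reissues AI MoveTo, except while IsBeingLaunched is set, which clears after a short delay.
; Within range of the player, it flags the jump tutorial unless already completed.
; At zero health, it once updates BP_GameMode's enemy count and currency, enables mesh physics, then destroys itself after a delay.
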(event Custom|TutoCheck
  (bind _asbp_first_person_character (Utilities|Casting|CastToBP_FirstPersonCharacter (Game|GetPlayerCharacter 0)))
  (if (< (Transformation|GetDistanceTo _asbp_first_person_character) 6e+02)
    (if (not (Variables|/Game/FirstPerson/Blueprints/BP_FirstPersonCharacter.BP_FirstPersonCharacter_C|GetJumpTutoComp _asbp_first_person_character))
      (Variables|/Game/FirstPerson/Blueprints/BP_FirstPersonCharacter.BP_FirstPersonCharacter_C|SetJumpTuto _asbp_first_person_character true))))

(event Custom|MoveToCrystal
  (bind _asbp_game_instance (Utilities|Casting|CastToBP_GameInstance (Game|GetGameInstance)))
  (AI|AIMoveTo self (Variables|/Game/FirstPerson/Blueprints/BP_GameInstance.BP_GameInstance_C|GetCrystalLocation _asbp_game_instance) 0 1.0 false))

(event EventBeginPlay
  (Components|Animation|PlayAnimation (Variables|Character|GetMesh) "/Game/Enemys/Small/Necro_Enemy_Small_Movement_Anim.Necro_Enemy_Small_Movement_Anim" true))

(event Collision|EventActorBeginOverlap
  (params (OtherActor :type Actor%20Object%20Reference)))

(event EventTick
  (params (DeltaSeconds :type Float%20%28single-precision%29))
  (if (<= (Variables|Default|GetHealth) 0.0)
    (bind _asbp_game_mode (Utilities|Casting|CastToBP_GameMode (Game|GetGameMode)))
    (Utilities|FlowControl|DoOnce false
      (:Completed
        (Variables|/Game/MiscBlueprints/BP_GameMode.BP_GameMode_C|SetEnemiesAlive _asbp_game_mode (- (Variables|/Game/MiscBlueprints/BP_GameMode.BP_GameMode_C|GetEnemiesAlive _asbp_game_mode) 1))
        (Variables|/Game/MiscBlueprints/BP_GameMode.BP_GameMode_C|SetCurrency _asbp_game_mode (+ (Variables|/Game/MiscBlueprints/BP_GameMode.BP_GameMode_C|GetCurrency _asbp_game_mode) 100))
        (Physics|SetSimulatePhysics (Variables|Character|GetMesh) true)
        (Utilities|FlowControl|Delay 3.0)
        (Actor|DestroyActor)))
    (elif (Variables|Default|GetisBeingLaunched)
      (Utilities|FlowControl|Delay 2.0)
      (Variables|Default|SetisBeingLaunched false)
      (else
        (CallFunction|MovetoCrystal)
        (CallFunction|TutoCheck)))))

(fn ConstructionScript)