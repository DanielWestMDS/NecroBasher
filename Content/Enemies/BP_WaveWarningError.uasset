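; Wave warning actor that lines a spline with copies of a chosen mesh and animates their height.
; Construction script spaces instances by mesh X bounds plus XOffset, rotating each toward the next point.
; Tick lerps the whole instanced component's Z between zero and YOffset, switching direction around a fixed CurrentHeight threshold with DoOnce gates.
; Only the rising branch advances AlphaTick by delta time; the falling branch adds zero.
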(event EventBeginPlay)

(event EventTick
  (params (DeltaSeconds :type Float%20%28single-precision%29))
  (if (< (Variables|Default|GetCurrentHeight) 1e+02)
    (Utilities|FlowControl|Sequence
      (:then_0
        (Utilities|FlowControl|DoOnce false :!label _label
          (:Completed
            (Variables|Default|SetAlphaTick 0.0))))
      (:then_1
        (if (> (Variables|Default|GetAlphaTick) 1.0)
          _
          (else
            (Variables|Default|SetAlphaTick (+ DeltaSeconds (Variables|Default|GetAlphaTick)))))
        (Transformation|SetRelativeTransform (Variables|Default|GetInstancedStaticMesh) (Math|Transform|MakeTransform (Math|Vector|MakeVector 0.0 0.0 (Math|Float|Lerp 0.0 (Variables|Default|GetYOffset) (Variables|Default|GetAlphaTick))) "0, 0, 0" "1.000000,1.000000,1.000000") false false)
        (Variables|Default|SetCurrentHeight (Math|Float|Lerp 0.0 (Variables|Default|GetYOffset) (Variables|Default|GetAlphaTick)))
        (goto _label_2 Reset)))
    (else
      (Utilities|FlowControl|Sequence
        (:then_0
          (Utilities|FlowControl|DoOnce false :!label _label_2
            (:Completed
              (Variables|Default|SetAlphaTick 0.0))))
        (:then_1
          (if (> (Variables|Default|GetAlphaTick) 1.0)
            _
            (else
              (Variables|Default|SetAlphaTick (+ 0.0 (Variables|Default|GetAlphaTick)))))
          (Transformation|SetRelativeTransform (Variables|Default|GetInstancedStaticMesh) (Math|Transform|MakeTransform (Math|Vector|MakeVector 0.0 0.0 (Math|Float|Lerp (Variables|Default|GetYOffset) 0.0 (Variables|Default|GetAlphaTick))) "0, 0, 0" "1.000000,1.000000,1.000000") false false)
          (Variables|Default|SetCurrentHeight (Math|Float|Lerp (Variables|Default|GetYOffset) 0.0 (Variables|Default|GetAlphaTick)))
          (goto _label Reset))))))

(fn ConstructionScript
  (bind _placedmesh (Variables|Default|GetPlacedMesh))
  (bind _returnvalue (StaticMesh|GetBoundingBox _placedmesh))
  (bind (_min _max) (Utilities|Struct|BreakBox _returnvalue))
  (Components|StaticMesh|SetStaticMesh (Variables|Default|GetInstancedStaticMesh) (Variables|Default|GetPlacedMesh))
  (bind _output_get (Variables|Default|SetSpacing (+ (.X (Math|Vector|BreakVector (- _max _min))) (Variables|Default|GetXOffset))))
  (bind _output_get_2 (LocalVariables|SetNumberOfInstances (Math|Float|Floor (/ (Spline|GetSplineLength (Variables|Default|GetSpline)) _output_get))))
  (for _index (range 0 _output_get_2)
    (Variables|Default|SetNumOfInstances (Math|Integer|Max(Integer) _index))
    (Components|InstancedStaticMesh|AddInstance (Variables|Default|GetInstancedStaticMesh) (Math|Transform|MakeTransform (CallFunction|GetLocationatIndex _index) (Math|Rotator|MakeRotfromX (- (CallFunction|GetLocationatIndex (+ _index 1)) (CallFunction|GetLocationatIndex _index)))) false)))

(fn GetLocationatIndex
  (params (A :type Integer))
  (return (Spline|GetLocationatDistanceAlongSpline (Variables|Default|GetSpline) (* A (Variables|Default|GetSpacing)) "Local")))