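; Enemy spawner that creates attack and speed enemies at its billboard during game-mode rounds.
; Tick initializes each round's spawn delays once via DoOnce, then, while in a round, waits a global delay and calls that round's spawn event.
; Spawning requires positive per-round and BP_GameMode counts, decrementing the latter before a per-type delay.
; Round 3's spawn call is disconnected, so only rounds 1 and 2 spawn.
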(event Custom|SpawnAttackEnemy
  ;[0.1094 0.1094 0.1094] Spawn attack enemy at spawner location
  (Variables|/Game/MiscBlueprints/BP_GameMode.BP_GameMode_C|SetNumAttackEnemiesToSpawn (stale EventTick _asbp_game_mode) (- (Variables|/Game/MiscBlueprints/BP_GameMode.BP_GameMode_C|GetNumAttackEnemiesToSpawn (stale EventTick _asbp_game_mode)) 1)) ; decrement num of attack enemies to be spawned
  (Utilities|FlowControl|Delay (Variables|Default|GetAttackEnemySpawnDelay))
  (Game|SpawnActorfromClass "/Game/Enemies/BP_Enemy.BP_Enemy_C" (Math|Transform|MakeTransform (Transformation|GetWorldLocation (Variables|Default|GetBillboard)) "0, 0, 0" "1.000000,1.000000,1.000000") "Undefined" "MultiplyWithRoot" 0 0))

(event Custom|SpawnSpeedEnemy
  ;[0.1094 0.1094 0.1094] Spawn speed enemy at spawner location
  (Variables|/Game/MiscBlueprints/BP_GameMode.BP_GameMode_C|SetNumSpeedEnemiesToSpawn (stale EventTick _asbp_game_mode) (- (Variables|/Game/MiscBlueprints/BP_GameMode.BP_GameMode_C|GetNumSpeedEnemiesToSpawn (stale EventTick _asbp_game_mode)) 1))
  (Utilities|FlowControl|Delay (Variables|Default|GetSpeedEnemySpawnDelay))
  (Game|SpawnActorfromClass "/Game/Enemies/BP_SpeedEnemy.BP_SpeedEnemy_C" (Math|Transform|MakeTransform (Transformation|GetWorldLocation (Variables|Default|GetBillboard)) "0, 0, 0" "1.000000,1.000000,1.000000") "Undefined" "MultiplyWithRoot" 0 0))

(event Custom|InitializeRound
  ;[0.1083 0.1083 0.1083] Initialize each round with proper enemy amounts with cast to gamemode
  (bind _asbp_game_mode (Utilities|Casting|CastToBP_GameMode (Game|GetGameMode)))
  (if (== (Variables|/Game/MiscBlueprints/BP_GameMode.BP_GameMode_C|GetCurrentRound _asbp_game_mode) 1)
    (Utilities|FlowControl|DoOnce false
      (:Completed
        (Variables|/Game/MiscBlueprints/BP_GameMode.BP_GameMode_C|SetNumAttackEnemiesToSpawn _asbp_game_mode (Variables|/Game/MiscBlueprints/BP_GameMode.BP_GameMode_C|GetNumAttackEnemiesToSpawn _asbp_game_mode))
        (Variables|/Game/MiscBlueprints/BP_GameMode.BP_GameMode_C|SetNumSpeedEnemiesToSpawn _asbp_game_mode (Variables|/Game/MiscBlueprints/BP_GameMode.BP_GameMode_C|GetNumSpeedEnemiesToSpawn _asbp_game_mode))
        (Variables|Default|SetGlobalSpawnDelay 2.0)
        (Variables|Default|SetAttackEnemySpawnDelay 2.0)
        (Variables|Default|SetSpeedEnemySpawnDelay 0.0)))
    (elif (== (Variables|/Game/MiscBlueprints/BP_GameMode.BP_GameMode_C|GetCurrentRound _asbp_game_mode) 2)
      (Utilities|FlowControl|DoOnce false
        (:Completed
          (Variables|/Game/MiscBlueprints/BP_GameMode.BP_GameMode_C|SetNumAttackEnemiesToSpawn _asbp_game_mode (Variables|/Game/MiscBlueprints/BP_GameMode.BP_GameMode_C|GetNumAttackEnemiesToSpawn _asbp_game_mode))
          (Variables|/Game/MiscBlueprints/BP_GameMode.BP_GameMode_C|SetNumSpeedEnemiesToSpawn _asbp_game_mode (Variables|/Game/MiscBlueprints/BP_GameMode.BP_GameMode_C|GetNumSpeedEnemiesToSpawn _asbp_game_mode))
          (Variables|Default|SetGlobalSpawnDelay 1.0)
          (Variables|Default|SetAttackEnemySpawnDelay 0.0)
          (Variables|Default|SetSpeedEnemySpawnDelay 0.0)))
      (elif (== (Variables|/Game/MiscBlueprints/BP_GameMode.BP_GameMode_C|GetCurrentRound _asbp_game_mode) 3)
        (Utilities|FlowControl|DoOnce false
          (:Completed
            (Variables|/Game/MiscBlueprints/BP_GameMode.BP_GameMode_C|SetNumAttackEnemiesToSpawn _asbp_game_mode (Variables|/Game/MiscBlueprints/BP_GameMode.BP_GameMode_C|GetNumAttackEnemiesToSpawn _asbp_game_mode))
            (Variables|/Game/MiscBlueprints/BP_GameMode.BP_GameMode_C|SetNumSpeedEnemiesToSpawn _asbp_game_mode (Variables|/Game/MiscBlueprints/BP_GameMode.BP_GameMode_C|GetNumSpeedEnemiesToSpawn _asbp_game_mode))
            (Variables|Default|SetGlobalSpawnDelay 0.0)
            (Variables|Default|SetAttackEnemySpawnDelay 0.0)
            (Variables|Default|SetSpeedEnemySpawnDelay 0.0)))))))

(event Custom|RoundComplete
  ;[0.1094 0.1094 0.1094] When round completes initialize the next round
  (CallFunction|InitializeRound))

(event Custom|Round1EnemySpawn
  ;[0.1094 0.1094 0.1094] Spawning Enemies in Round 1
  (bind _asbp_game_mode (Utilities|Casting|CastToBP_GameMode (Game|GetGameMode)))
  (Utilities|FlowControl|Sequence
    (:then_0
      (if (and (> (Variables|Default|GetRound1AttackEnemiesToSpawn) 0) (> (Variables|/Game/MiscBlueprints/BP_GameMode.BP_GameMode_C|GetNumAttackEnemiesToSpawn _asbp_game_mode) 0))
        (CallFunction|SpawnAttackEnemy)))
    (:then_1
      (if (and (> (Variables|/Game/MiscBlueprints/BP_GameMode.BP_GameMode_C|GetNumSpeedEnemiesToSpawn _asbp_game_mode) 0) (> (Variables|Default|GetRound1SpeedEnemiesToSpawn) 0))
        (CallFunction|SpawnSpeedEnemy)))))

(event Custom|Round2EnemySpawn
  ;[0.1094 0.1094 0.1094] Spawning Enemies in Round 2
  (Utilities|FlowControl|Sequence
    (:then_0
      (if (and (> (Variables|Default|GetRound2AttackEnemiesToSpawn) 0) (> (Variables|/Game/MiscBlueprints/BP_GameMode.BP_GameMode_C|GetNumAttackEnemiesToSpawn (stale Custom|Round1EnemySpawn _asbp_game_mode)) 0))
        (CallFunction|SpawnAttackEnemy)))
    (:then_1
      (if (and (> (Variables|/Game/MiscBlueprints/BP_GameMode.BP_GameMode_C|GetNumSpeedEnemiesToSpawn (stale Custom|Round1EnemySpawn _asbp_game_mode)) 0) (> (Variables|Default|GetRound2SpeedEnemiesToSpawn) 0))
        (CallFunction|SpawnSpeedEnemy)))))

(event Custom|Round3EnemySpawn
  ;[0.1094 0.1094 0.1094] Spawning Enemies in Round 3
  (Utilities|FlowControl|Sequence
    (:then_0
      (if (and (> (Variables|Default|GetRound3AttackEnemiesToSpawn) 0) (> (Variables|/Game/MiscBlueprints/BP_GameMode.BP_GameMode_C|GetNumAttackEnemiesToSpawn (stale Custom|Round1EnemySpawn _asbp_game_mode)) 0))
        (CallFunction|SpawnAttackEnemy)))
    (:then_1
      (if (and (> (Variables|/Game/MiscBlueprints/BP_GameMode.BP_GameMode_C|GetNumSpeedEnemiesToSpawn (stale Custom|Round1EnemySpawn _asbp_game_mode)) 0) (> (Variables|Default|GetRound3SpeedEnemiesToSpawn) 0))
        (CallFunction|SpawnSpeedEnemy)))))

(event EventTick
  (params (DeltaSeconds :type Float%20%28single-precision%29))
  (CallFunction|InitializeRound)
  (bind _asbp_game_mode (Utilities|Casting|CastToBP_GameMode (Game|GetGameMode)))
  ;[0.1094 0.1094 0.1094] If player is in round spawn enemies
  (if (Variables|/Game/MiscBlueprints/BP_GameMode.BP_GameMode_C|GetInRound _asbp_game_mode)
    (Utilities|FlowControl|Delay (Variables|Default|GetGlobalSpawnDelay)) ; Spawn delay on spawner if you wanted to \nsay stagger certain lanes
    ;[0.1094 0.1094 0.1094] Spawn enemies based on round
    (Utilities|FlowControl|Sequence
      (:then_0
        (if (== (Variables|/Game/MiscBlueprints/BP_GameMode.BP_GameMode_C|GetCurrentRound _asbp_game_mode) 1)
          (CallFunction|Round1EnemySpawn)))
      (:then_1
        (if (== (Variables|/Game/MiscBlueprints/BP_GameMode.BP_GameMode_C|GetCurrentRound _asbp_game_mode) 2)
          (CallFunction|Round2EnemySpawn))))
    (else
      (CallFunction|RoundComplete))))

(fn ConstructionScript)