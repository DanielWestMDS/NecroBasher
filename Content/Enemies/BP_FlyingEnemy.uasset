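; Flying enemy that follows a randomly picked spline, shoots at the player and shows a warning widget.
; Tick advances spline movement, blending rotation with lerps, and triggers timed attacks and a skill tutorial flag when the player is near.
; Attacks turn toward the player, then after a delay spawn a projectile and directly deduct a life.
; Death updates BP_GameMode's enemy count and currency, plays effects and destroys the actor.
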(event Custom|PickSpline
  ;[0.1094 0.1094 0.1094] Event to randomly pick a spline from spline array
  (Variables|References|SetMovementSpline (Utilities|Array|Get(acopy) (Variables|References|GetSplineArrayReference) (Math|Random|RandomInteger (Variables|Default|GetSplineMaxValue)))))

(event Custom|ProjectileAttackPlayer
  (bind _returnvalue (Transformation|GetActorLocation))
  (bind _player_reference (Variables|References|GetPlayer%20Reference))
  ;[0.1094 0.1094 0.1094] ProjectileAttack
  (Variables|Default|SetSplineTurningTick 0.0)
  (Variables|Default|SetIsShooting true)
  (CallFunction|RotateEnemy)
  (Utilities|FlowControl|Delay 2.0)
  (Audio|PlaySoundatLocation "/Game/Sound/Laser_Shoot_New.Laser_Shoot_New" _returnvalue "0, 0, 0" 1.0 1.0 0.0 0 0 0 0)
  (Game|SpawnActorfromClass "/Game/Enemies/BP_EnemyProjectile.BP_EnemyProjectile_C" (Math|Transform|MakeTransform _returnvalue (Math|Rotator|FindLookatRotation _returnvalue (Transformation|GetWorldLocation (Variables|/Script/Engine.Actor|GetRootComponent (Variables|References|GetPlayer%20Reference)))) "1.000000,1.000000,1.000000") "Undefined" "MultiplyWithRoot" 0 0)
  (Variables|/Game/FirstPerson/Blueprints/BP_FirstPersonCharacter.BP_FirstPersonCharacter_C|SetLives _player_reference (- (Variables|/Game/FirstPerson/Blueprints/BP_FirstPersonCharacter.BP_FirstPersonCharacter_C|GetLives _player_reference) 1))
  (Variables|/Game/FirstPerson/Blueprints/BP_FirstPersonCharacter.BP_FirstPersonCharacter_C|SetHit _player_reference 1.0))

(event Custom|EnemyDeath
  (Development|PrintString "flying enemy died")
  (bind _asbp_game_mode (Utilities|Casting|CastToBP_GameMode (Game|GetGameMode)))
  (Utilities|FlowControl|DoOnce false
    (:Completed
      ;[0.1094 0.1094 0.1094] Decrement Global Enemy count
      (Variables|/Game/MiscBlueprints/BP_GameMode.BP_GameMode_C|SetEnemiesAlive _asbp_game_mode (- (Variables|/Game/MiscBlueprints/BP_GameMode.BP_GameMode_C|GetEnemiesAlive _asbp_game_mode) 1))
      ;[0.1094 0.1094 0.1094] Give Currency To Player
      (Variables|/Game/MiscBlueprints/BP_GameMode.BP_GameMode_C|SetCurrency _asbp_game_mode (+ (Variables|/Game/MiscBlueprints/BP_GameMode.BP_GameMode_C|GetCurrency _asbp_game_mode) 100))
      (Utilities|FlowControl|Delay 0.2)
      ;[0.1094 0.1094 0.1094] DO NOT CHANGE THIS WHOLE GAME WILL BREAK IF YOU CHANGE THIS DO NOT CHANGE
      (Physics|SetSimulatePhysics (Variables|Character|GetMesh) false)
      (Utilities|FlowControl|Delay 0.0)
      (Niagara|SpawnSystematLocation "/Game/VFX_BEAM/VFX_Enemy_Death.VFX_Enemy_Death" (Transformation|GetWorldLocation (Variables|Character|GetMesh)) "0, 0, 0" "1.200000,1.200000,1.200000")
      (Audio|PlaySoundatLocation "/Game/Sound/enemyDie.enemyDie" "0, 0, 0" "0, 0, 0" 1.0 1.0 0.0 0 0 0 0)
      (Utilities|FlowControl|Delay 0.1)
      (Actor|DestroyActor))))

(event Custom|RotateEnemy
  (bind _returnvalue (Transformation|GetActorLocation))
  (bind _movementspline (Variables|References|GetMovementSpline))
  (bind _player_reference (Variables|References|GetPlayer%20Reference))
  (bind _distancealongspline (Variables|Movement|GetDistanceAlongSpline))
  (bind _returnvalue_2 (Transformation|GetActorLocation _player_reference))
  (bind _spline (Variables|/Game/Enemies/Splines/BP_FlyingEnemySpline.BP_FlyingEnemySpline_C|GetSpline _movementspline))
  (bind _returnvalue_3 (Spline|GetRotationatDistanceAlongSpline _spline _distancealongspline "World"))
  (bind _returnvalue_4 (Math|Rotator|FindLookatRotation _returnvalue _returnvalue_2))
  ;[0.1844 0.1844 0.1844] Rotate Enemy towards player position
  (if (> (Variables|Default|GetProjectileTurningTick) 1.0)
    _
    (else
      (Variables|Default|SetProjectileTurningTick (+ (Utilities|Time|GetWorldDeltaSeconds) (Variables|Default|GetProjectileTurningTick)))))
  (Transformation|SetActorRotation (Math|Rotator|MakeRotator (.roll (Math|Rotator|Lerp(Rotator) (Math|Rotator|MakeRotator (.roll _returnvalue_3) (.pitch _returnvalue_3) (.yaw _returnvalue_3)) (Math|Rotator|MakeRotator (.roll _returnvalue_4) (.pitch _returnvalue_4) (.yaw _returnvalue_4)) (Variables|Default|GetProjectileTurningTick) true)) (.pitch (Math|Rotator|Lerp(Rotator) (Math|Rotator|MakeRotator (.roll _returnvalue_3) (.pitch _returnvalue_3) (.yaw _returnvalue_3)) (Math|Rotator|MakeRotator (.roll _returnvalue_4) (.pitch _returnvalue_4) (.yaw _returnvalue_4)) (Variables|Default|GetProjectileTurningTick) true)) (.yaw (Math|Rotator|Lerp(Rotator) (Math|Rotator|MakeRotator (.roll _returnvalue_3) (.pitch _returnvalue_3) (.yaw _returnvalue_3)) (Math|Rotator|MakeRotator (.roll _returnvalue_4) (.pitch _returnvalue_4) (.yaw _returnvalue_4)) (Variables|Default|GetProjectileTurningTick) true)))))

(event Custom|MovementAlongSpline
  (bind _isshooting (Variables|Default|GetIsShooting))
  (bind _movementspline (Variables|References|GetMovementSpline))
  ;[0.1844 0.1844 0.1844] Movement for enemy along spline
  (Utilities|FlowControl|Sequence
    (:then_0
      (if (not (Variables|Default|GetIsShooting))
        (Variables|Default|SetProjectileTurningTick 0.0)))
    (:then_1
      (Variables|Movement|SetDistanceAlongSpline (+ (* (Utilities|Time|GetWorldDeltaSeconds) (Variables|Movement|GetSplineSpeed)) (Variables|Movement|GetDistanceAlongSpline)))
      (if (> (Variables|Default|GetSplineTurningTick) 1.0)
        _
        (else
          (Variables|Default|SetSplineTurningTick (+ (Utilities|Time|GetWorldDeltaSeconds) (Variables|Default|GetSplineTurningTick)))))
      (Transformation|SetActorLocation (Spline|GetLocationatDistanceAlongSpline (Variables|/Game/Enemies/Splines/BP_FlyingEnemySpline.BP_FlyingEnemySpline_C|GetSpline _movementspline) (Variables|Movement|GetDistanceAlongSpline) "World") true false)
      (bind _output_get (Variables|Default|SetLastSpline (Spline|GetLocationatDistanceAlongSpline (Variables|/Game/Enemies/Splines/BP_FlyingEnemySpline.BP_FlyingEnemySpline_C|GetSpline _movementspline) (Variables|Movement|GetDistanceAlongSpline) "World")))
      (if (not _isshooting)
        (Development|PrintString (Utilities|String|ToString(Boolean) _isshooting))
        (Transformation|SetActorRotation (Math|Rotator|Lerp(Rotator) (Math|Rotator|FindLookatRotation (Transformation|GetActorLocation) (Transformation|GetActorLocation (Variables|References|GetPlayer%20Reference))) (Spline|GetRotationatDistanceAlongSpline (Variables|/Game/Enemies/Splines/BP_FlyingEnemySpline.BP_FlyingEnemySpline_C|GetSpline _movementspline) (Variables|Movement|GetDistanceAlongSpline) "World") (Variables|Default|GetSplineTurningTick) true))
        (Utilities|FlowControl|DoOnce false
          (:Completed
            (Variables|Default|SetLastSpline (Transformation|GetActorLocation))))))))

(event EventBeginPlay
  ;[0.1094 0.1094 0.1094] Begin Play for player reference
  (Variables|Default|SetHealth 1e+01)
  (bind _asbp_first_person_character (Utilities|Casting|CastToBP_FirstPersonCharacter (Game|GetPlayerCharacter 0)))
  (Variables|References|SetPlayer%20Reference _asbp_first_person_character)
  ;[1 1 1] Locator UI
  (bind _returnvalue (UserInterface|CreateWidget "/Game/UI/WB_FlyingWarning.WB_FlyingWarning_C" (Game|GetPlayerController 0)))
  (bind _output_get (Variables|Default|SetWarningIcon _returnvalue))
  (Variables|/Game/UI/WB_FlyingWarning.WB_FlyingWarning_C|SetFlyingEnemy _output_get self)
  (UserInterface|Viewport|AddtoViewport _output_get 0))

(event EventTick
  (params (DeltaSeconds :type Float%20%28single-precision%29))
  ;[0.1094 0.1094 0.1094] Main Event Tick
  (Development|PrintString (Utilities|String|ToString(Float) (Variables|Movement|GetDistanceAlongSpline)))
  (Utilities|FlowControl|Sequence
    (:then_0
      (Utilities|FlowControl|DoOnce false
        (:Completed
          (CallFunction|PickSpline)
          (Variables|Default|SetLastSpline (Transformation|GetActorLocation)))))
    (:then_1
      (if (not (Variables|Default|GetIsBeingLaunched))
        (if (< (Transformation|GetDistanceTo (Variables|References|GetPlayer%20Reference)) 1e+03)
          (if (<= (Variables|Default|GetProjectileTimer) 0.0)
            (CallFunction|ProjectileAttackPlayer)
            (Variables|Default|SetProjectileTimer 5.0)
            (CallFunction|MovementAlongSpline :!label _label))
          (else
            (Variables|Default|SetIsShooting false)
            (goto _label)))))
    (:then_2
      (bind _asbp_first_person_character (Utilities|Casting|CastToBP_FirstPersonCharacter (Game|GetPlayerCharacter 0)))
      (if (< (Transformation|GetDistanceTo _asbp_first_person_character) 1e+03)
        (if (not (Variables|/Game/FirstPerson/Blueprints/BP_FirstPersonCharacter.BP_FirstPersonCharacter_C|GetSkillTutoComp _asbp_first_person_character))
          (Variables|/Game/FirstPerson/Blueprints/BP_FirstPersonCharacter.BP_FirstPersonCharacter_C|SetSkillTuto _asbp_first_person_character true))))
    (:then_3
      (Variables|Default|SetProjectileTimer (- (Variables|Default|GetProjectileTimer) DeltaSeconds)))))

(fn ConstructionScript)