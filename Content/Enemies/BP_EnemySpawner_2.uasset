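; Enemy spawner that spawns attack and speed enemies at its billboard across eight rounds.
; Tick applies each round's timings once and, during a round, routes to that round's spawn event after a lane-staggering delay.
; Delay nodes pace spawns, which decrement GameMode totals and, except in round 1, per-round spawner quotas.
; Rounds 2-3, 5-6 and 8 reuse GameMode references cached by rounds 1, 4 and 7.
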(event Custom|SpawnAttackEnemy
  (bind _asbp_game_mode (Utilities|Casting|CastToBP_GameMode (Game|GetGameMode)))
  (Utilities|FlowControl|Delay (Variables|Default|GetAttackEnemySpawnDelay))
  (Game|SpawnActorfromClass "/Game/Enemies/BP_Enemy.BP_Enemy_C" (Math|Transform|MakeTransform (Transformation|GetWorldLocation (Variables|Default|GetBillboard)) "0, 0, 0" "1.000000,1.000000,1.000000") "Undefined" "MultiplyWithRoot" 0 0)
  (Variables|/Game/MiscBlueprints/BP_GameMode.BP_GameMode_C|SetNumAttackEnemiesToSpawn _asbp_game_mode (- (Variables|/Game/MiscBlueprints/BP_GameMode.BP_GameMode_C|GetNumAttackEnemiesToSpawn _asbp_game_mode) 1)) ; decrement num of attack enemies to be spawned
  (Utilities|FlowControl|Sequence
    (:then_0
      (if (== (Variables|/Game/MiscBlueprints/BP_GameMode.BP_GameMode_C|GetCurrentRound _asbp_game_mode) 1)
        _))
    (:then_1
      (if (== (Variables|/Game/MiscBlueprints/BP_GameMode.BP_GameMode_C|GetCurrentRound _asbp_game_mode) 2)
        (Variables|Default|SetRound2AttackEnemiesToSpawn (- (Variables|Default|GetRound2AttackEnemiesToSpawn) 1))))
    (:then_2
      (if (== (Variables|/Game/MiscBlueprints/BP_GameMode.BP_GameMode_C|GetCurrentRound _asbp_game_mode) 3)
        (Variables|Default|SetRound3AttackEnemiesToSpawn (- (Variables|Default|GetRound3AttackEnemiesToSpawn) 1))))
    (:then_3
      (if (== (Variables|/Game/MiscBlueprints/BP_GameMode.BP_GameMode_C|GetCurrentRound _asbp_game_mode) 4)
        (Variables|Default|SetRound4AttackEnemiesToSpawn (- (Variables|Default|GetRound4AttackEnemiesToSpawn) 1))))
    (:then_4
      (if (== (Variables|/Game/MiscBlueprints/BP_GameMode.BP_GameMode_C|GetCurrentRound _asbp_game_mode) 5)
        (Variables|Default|SetRound5AttackEnemiesToSpawn (- (Variables|Default|GetRound5AttackEnemiesToSpawn) 1))))
    (:then_5
      (if (== (Variables|/Game/MiscBlueprints/BP_GameMode.BP_GameMode_C|GetCurrentRound _asbp_game_mode) 6)
        (Variables|Default|SetRound6AttackEnemiesToSpawn (- (Variables|Default|GetRound6AttackEnemiesToSpawn) 1))))
    (:then_6
      (if (== (Variables|/Game/MiscBlueprints/BP_GameMode.BP_GameMode_C|GetCurrentRound _asbp_game_mode) 7)
        (Variables|Default|SetRound7AttackEnemiesToSpawn (- (Variables|Default|GetRound7AttackEnemiesToSpawn) 1))))
    (:then_7
      (if (== (Variables|/Game/MiscBlueprints/BP_GameMode.BP_GameMode_C|GetCurrentRound _asbp_game_mode) 8)
        (Variables|Default|SetRound8AttackEnemiesToSpawn (- (Variables|Default|GetRound8AttackEnemiesToSpawn) 1))))))

(event Custom|SpawnSpeedEnemy
  ;[0.1094 0.1094 0.1094] Spawn speed enemy at spawner location
  (bind _asbp_game_mode (Utilities|Casting|CastToBP_GameMode (Game|GetGameMode)))
  (Utilities|FlowControl|Delay (Variables|Default|GetSpeedEnemySpawnDelay))
  (Game|SpawnActorfromClass "/Game/Enemies/BP_SpeedEnemy.BP_SpeedEnemy_C" (Math|Transform|MakeTransform (Transformation|GetWorldLocation (Variables|Default|GetBillboard)) "0, 0, 0" "1.000000,1.000000,1.000000") "Undefined" "MultiplyWithRoot" 0 0)
  (Variables|/Game/MiscBlueprints/BP_GameMode.BP_GameMode_C|SetNumSpeedEnemiesToSpawn _asbp_game_mode (- (Variables|/Game/MiscBlueprints/BP_GameMode.BP_GameMode_C|GetNumSpeedEnemiesToSpawn _asbp_game_mode) 1))
  (Utilities|FlowControl|Sequence
    (:then_0
      (if (== (Variables|/Game/MiscBlueprints/BP_GameMode.BP_GameMode_C|GetCurrentRound _asbp_game_mode) 1)
        _))
    (:then_1
      (if (== (Variables|/Game/MiscBlueprints/BP_GameMode.BP_GameMode_C|GetCurrentRound _asbp_game_mode) 2)
        (Variables|Default|SetRound2SpeedEnemiesToSpawn (- (Variables|Default|GetRound2SpeedEnemiesToSpawn) 1))))
    (:then_2
      (if (== (Variables|/Game/MiscBlueprints/BP_GameMode.BP_GameMode_C|GetCurrentRound _asbp_game_mode) 3)
        (Variables|Default|SetRound3SpeedEnemiesToSpawn (- (Variables|Default|GetRound3SpeedEnemiesToSpawn) 1))))
    (:then_3
      (if (== (Variables|/Game/MiscBlueprints/BP_GameMode.BP_GameMode_C|GetCurrentRound _asbp_game_mode) 4)
        (Variables|Default|SetRound4SpeedEnemiesToSpawn (- (Variables|Default|GetRound4SpeedEnemiesToSpawn) 1))))
    (:then_4
      (if (== (Variables|/Game/MiscBlueprints/BP_GameMode.BP_GameMode_C|GetCurrentRound _asbp_game_mode) 5)
        (Variables|Default|SetRound5SpeedEnemiesToSpawn (- (Variables|Default|GetRound5SpeedEnemiesToSpawn) 1))))
    (:then_5
      (if (== (Variables|/Game/MiscBlueprints/BP_GameMode.BP_GameMode_C|GetCurrentRound _asbp_game_mode) 6)
        (Variables|Default|SetRound6SpeedEnemiesToSpawn (- (Variables|Default|GetRound6SpeedEnemiesToSpawn) 1))))
    (:then_6
      (if (== (Variables|/Game/MiscBlueprints/BP_GameMode.BP_GameMode_C|GetCurrentRound _asbp_game_mode) 7)
        (Variables|Default|SetRound7SpeedEnemiesToSpawn (- (Variables|Default|GetRound7SpeedEnemiesToSpawn) 1))))
    (:then_7
      (if (== (Variables|/Game/MiscBlueprints/BP_GameMode.BP_GameMode_C|GetCurrentRound _asbp_game_mode) 8)
        (Variables|Default|SetRound8SpeedEnemiesToSpawn (- (Variables|Default|GetRound8SpeedEnemiesToSpawn) 1))))))

(event Custom|Round4EnemySpawn
  ;[0.1094 0.1094 0.1094] Spawning Enemies in Round 4
  (bind _asbp_game_mode (Utilities|Casting|CastToBP_GameMode (Game|GetGameMode)))
  (Utilities|FlowControl|Sequence
    (:then_0
      (if (and (> (Variables|Default|GetRound4AttackEnemiesToSpawn) 0) (> (Variables|/Game/MiscBlueprints/BP_GameMode.BP_GameMode_C|GetNumAttackEnemiesToSpawn _asbp_game_mode) 0))
        (CallFunction|SpawnAttackEnemy)))
    (:then_1
      (if (and (> (Variables|/Game/MiscBlueprints/BP_GameMode.BP_GameMode_C|GetNumSpeedEnemiesToSpawn _asbp_game_mode) 0) (> (Variables|Default|GetRound4SpeedEnemiesToSpawn) 0))
        (CallFunction|SpawnSpeedEnemy)))))

(event Custom|Round5EnemySpawn
  ;[0.1094 0.1094 0.1094] Spawning Enemies in Round 5
  (Utilities|FlowControl|Sequence
    (:then_0
      (if (and (> (Variables|Default|GetRound5AttackEnemiesToSpawn) 0) (> (Variables|/Game/MiscBlueprints/BP_GameMode.BP_GameMode_C|GetNumAttackEnemiesToSpawn (stale Custom|Round4EnemySpawn _asbp_game_mode)) 0))
        (CallFunction|SpawnAttackEnemy)))
    (:then_1
      (if (and (> (Variables|/Game/MiscBlueprints/BP_GameMode.BP_GameMode_C|GetNumSpeedEnemiesToSpawn (stale Custom|Round4EnemySpawn _asbp_game_mode)) 0) (> (Variables|Default|GetRound5SpeedEnemiesToSpawn) 0))
        (CallFunction|SpawnSpeedEnemy)))))

(event Custom|InitializeRound
  ;[0.1083 0.1083 0.1083] Initialize each round with proper enemy amounts with cast to gamemode
  (bind _asbp_game_mode (Utilities|Casting|CastToBP_GameMode (Game|GetGameMode)))
  (if (== (Variables|/Game/MiscBlueprints/BP_GameMode.BP_GameMode_C|GetCurrentRound _asbp_game_mode) 1)
    (Utilities|FlowControl|DoOnce false
      (:Completed
        (Variables|/Game/MiscBlueprints/BP_GameMode.BP_GameMode_C|SetNumAttackEnemiesToSpawn _asbp_game_mode (Variables|/Game/MiscBlueprints/BP_GameMode.BP_GameMode_C|GetNumAttackEnemiesToSpawn _asbp_game_mode))
        (Variables|/Game/MiscBlueprints/BP_GameMode.BP_GameMode_C|SetNumSpeedEnemiesToSpawn _asbp_game_mode (Variables|/Game/MiscBlueprints/BP_GameMode.BP_GameMode_C|GetNumSpeedEnemiesToSpawn _asbp_game_mode))
        (Variables|Default|SetGlobalSpawnDelay 2.0)
        (Variables|Default|SetAttackEnemySpawnDelay 2.0)
        (Variables|Default|SetSpeedEnemySpawnDelay 0.2)
        (Variables|Default|SetHasGlobalDelayHappened false)))
    (elif (== (Variables|/Game/MiscBlueprints/BP_GameMode.BP_GameMode_C|GetCurrentRound _asbp_game_mode) 2)
      (Utilities|FlowControl|DoOnce false
        (:Completed
          (Variables|/Game/MiscBlueprints/BP_GameMode.BP_GameMode_C|SetNumAttackEnemiesToSpawn _asbp_game_mode (Variables|/Game/MiscBlueprints/BP_GameMode.BP_GameMode_C|GetNumAttackEnemiesToSpawn _asbp_game_mode))
          (Variables|/Game/MiscBlueprints/BP_GameMode.BP_GameMode_C|SetNumSpeedEnemiesToSpawn _asbp_game_mode (Variables|/Game/MiscBlueprints/BP_GameMode.BP_GameMode_C|GetNumSpeedEnemiesToSpawn _asbp_game_mode))
          (Variables|Default|SetGlobalSpawnDelay 5.0)
          (Variables|Default|SetAttackEnemySpawnDelay 1.0)
          (Variables|Default|SetSpeedEnemySpawnDelay 2.0)
          (Variables|Default|SetHasGlobalDelayHappened false)))
      (elif (== (Variables|/Game/MiscBlueprints/BP_GameMode.BP_GameMode_C|GetCurrentRound _asbp_game_mode) 3)
        (Utilities|FlowControl|DoOnce false
          (:Completed
            (Variables|/Game/MiscBlueprints/BP_GameMode.BP_GameMode_C|SetNumAttackEnemiesToSpawn _asbp_game_mode (Variables|/Game/MiscBlueprints/BP_GameMode.BP_GameMode_C|GetNumAttackEnemiesToSpawn _asbp_game_mode))
            (Variables|/Game/MiscBlueprints/BP_GameMode.BP_GameMode_C|SetNumSpeedEnemiesToSpawn _asbp_game_mode (Variables|/Game/MiscBlueprints/BP_GameMode.BP_GameMode_C|GetNumSpeedEnemiesToSpawn _asbp_game_mode))
            (Variables|Default|SetGlobalSpawnDelay 3.0)
            (Variables|Default|SetAttackEnemySpawnDelay 1.0)
            (Variables|Default|SetSpeedEnemySpawnDelay 1.0)
            (Variables|Default|SetHasGlobalDelayHappened false)))
        (elif (== (Variables|/Game/MiscBlueprints/BP_GameMode.BP_GameMode_C|GetCurrentRound _asbp_game_mode) 4)
          (Utilities|FlowControl|DoOnce false
            (:Completed
              (Variables|/Game/MiscBlueprints/BP_GameMode.BP_GameMode_C|SetNumAttackEnemiesToSpawn _asbp_game_mode (Variables|/Game/MiscBlueprints/BP_GameMode.BP_GameMode_C|GetNumAttackEnemiesToSpawn _asbp_game_mode))
              (Variables|/Game/MiscBlueprints/BP_GameMode.BP_GameMode_C|SetNumSpeedEnemiesToSpawn _asbp_game_mode (Variables|/Game/MiscBlueprints/BP_GameMode.BP_GameMode_C|GetNumSpeedEnemiesToSpawn _asbp_game_mode))
              (Variables|Default|SetGlobalSpawnDelay 3.0)
              (Variables|Default|SetAttackEnemySpawnDelay 1.0)
              (Variables|Default|SetSpeedEnemySpawnDelay 1.0)
              (Variables|Default|SetHasGlobalDelayHappened false)))
          (elif (== (Variables|/Game/MiscBlueprints/BP_GameMode.BP_GameMode_C|GetCurrentRound _asbp_game_mode) 5)
            (Utilities|FlowControl|DoOnce false
              (:Completed
                (Variables|/Game/MiscBlueprints/BP_GameMode.BP_GameMode_C|SetNumAttackEnemiesToSpawn _asbp_game_mode (Variables|/Game/MiscBlueprints/BP_GameMode.BP_GameMode_C|GetNumAttackEnemiesToSpawn _asbp_game_mode))
                (Variables|/Game/MiscBlueprints/BP_GameMode.BP_GameMode_C|SetNumSpeedEnemiesToSpawn _asbp_game_mode (Variables|/Game/MiscBlueprints/BP_GameMode.BP_GameMode_C|GetNumSpeedEnemiesToSpawn _asbp_game_mode))
                (Variables|Default|SetGlobalSpawnDelay 3.0)
                (Variables|Default|SetAttackEnemySpawnDelay 1.0)
                (Variables|Default|SetSpeedEnemySpawnDelay 1.0)
                (Variables|Default|SetHasGlobalDelayHappened false)))
            (elif (== (Variables|/Game/MiscBlueprints/BP_GameMode.BP_GameMode_C|GetCurrentRound _asbp_game_mode) 6)
              (Utilities|FlowControl|DoOnce false
                (:Completed
                  (Variables|/Game/MiscBlueprints/BP_GameMode.BP_GameMode_C|SetNumAttackEnemiesToSpawn _asbp_game_mode (Variables|/Game/MiscBlueprints/BP_GameMode.BP_GameMode_C|GetNumAttackEnemiesToSpawn _asbp_game_mode))
                  (Variables|/Game/MiscBlueprints/BP_GameMode.BP_GameMode_C|SetNumSpeedEnemiesToSpawn _asbp_game_mode (Variables|/Game/MiscBlueprints/BP_GameMode.BP_GameMode_C|GetNumSpeedEnemiesToSpawn _asbp_game_mode))
                  (Variables|Default|SetGlobalSpawnDelay 3.0)
                  (Variables|Default|SetAttackEnemySpawnDelay 1.0)
                  (Variables|Default|SetSpeedEnemySpawnDelay 1.0)
                  (Variables|Default|SetHasGlobalDelayHappened false)))
              (elif (== (Variables|/Game/MiscBlueprints/BP_GameMode.BP_GameMode_C|GetCurrentRound _asbp_game_mode) 7)
                (Utilities|FlowControl|DoOnce false
                  (:Completed
                    (Variables|/Game/MiscBlueprints/BP_GameMode.BP_GameMode_C|SetNumAttackEnemiesToSpawn _asbp_game_mode (Variables|/Game/MiscBlueprints/BP_GameMode.BP_GameMode_C|GetNumAttackEnemiesToSpawn _asbp_game_mode))
                    (Variables|/Game/MiscBlueprints/BP_GameMode.BP_GameMode_C|SetNumSpeedEnemiesToSpawn _asbp_game_mode (Variables|/Game/MiscBlueprints/BP_GameMode.BP_GameMode_C|GetNumSpeedEnemiesToSpawn _asbp_game_mode))
                    (Variables|Default|SetGlobalSpawnDelay 3.0)
                    (Variables|Default|SetAttackEnemySpawnDelay 1.0)
                    (Variables|Default|SetSpeedEnemySpawnDelay 1.0)
                    (Variables|Default|SetHasGlobalDelayHappened false)))
                (elif (== (Variables|/Game/MiscBlueprints/BP_GameMode.BP_GameMode_C|GetCurrentRound _asbp_game_mode) 8)
                  (Utilities|FlowControl|DoOnce false
                    (:Completed
                      (Variables|/Game/MiscBlueprints/BP_GameMode.BP_GameMode_C|SetNumAttackEnemiesToSpawn _asbp_game_mode (Variables|/Game/MiscBlueprints/BP_GameMode.BP_GameMode_C|GetNumAttackEnemiesToSpawn _asbp_game_mode))
                      (Variables|/Game/MiscBlueprints/BP_GameMode.BP_GameMode_C|SetNumSpeedEnemiesToSpawn _asbp_game_mode (Variables|/Game/MiscBlueprints/BP_GameMode.BP_GameMode_C|GetNumSpeedEnemiesToSpawn _asbp_game_mode))
                      (Variables|Default|SetGlobalSpawnDelay 3.0)
                      (Variables|Default|SetAttackEnemySpawnDelay 1.0)
                      (Variables|Default|SetSpeedEnemySpawnDelay 1.0)
                      (Variables|Default|SetHasGlobalDelayHappened false))))))))))))

(event Custom|RoundComplete
  ;[0.1094 0.1094 0.1094] When round completes initialize the next round
  (CallFunction|InitializeRound))

(event Custom|Round1EnemySpawn
  ;[0.1094 0.1094 0.1094] Spawning Enemies in Round 1
  (bind _asbp_game_mode (Utilities|Casting|CastToBP_GameMode (Game|GetGameMode)))
  (Utilities|FlowControl|Sequence
    (:then_0
      (if (and (> (Variables|Default|GetRound1AttackEnemiesToSpawn) 0) (> (Variables|/Game/MiscBlueprints/BP_GameMode.BP_GameMode_C|GetNumAttackEnemiesToSpawn _asbp_game_mode) 0))
        (CallFunction|SpawnAttackEnemy)))
    (:then_1
      (if (and (> (Variables|/Game/MiscBlueprints/BP_GameMode.BP_GameMode_C|GetNumSpeedEnemiesToSpawn _asbp_game_mode) 0) (> (Variables|Default|GetRound1SpeedEnemiesToSpawn) 0))
        (CallFunction|SpawnSpeedEnemy)))))

(event Custom|Round7EnemySpawn
  ;[0.1094 0.1094 0.1094] Spawning Enemies in Round 7
  (bind _asbp_game_mode (Utilities|Casting|CastToBP_GameMode (Game|GetGameMode)))
  (Utilities|FlowControl|Sequence
    (:then_0
      (if (and (> (Variables|Default|GetRound7AttackEnemiesToSpawn) 0) (> (Variables|/Game/MiscBlueprints/BP_GameMode.BP_GameMode_C|GetNumAttackEnemiesToSpawn _asbp_game_mode) 0))
        (CallFunction|SpawnAttackEnemy)))
    (:then_1
      (if (and (> (Variables|/Game/MiscBlueprints/BP_GameMode.BP_GameMode_C|GetNumSpeedEnemiesToSpawn _asbp_game_mode) 0) (> (Variables|Default|GetRound7SpeedEnemiesToSpawn) 0))
        (CallFunction|SpawnSpeedEnemy)))))

(event Custom|Round8EnemySpawn
  ;[0.1094 0.1094 0.1094] Spawning Enemies in Round 8
  (Utilities|FlowControl|Sequence
    (:then_0
      (if (and (> (Variables|Default|GetRound8AttackEnemiesToSpawn) 0) (> (Variables|/Game/MiscBlueprints/BP_GameMode.BP_GameMode_C|GetNumAttackEnemiesToSpawn (stale Custom|Round7EnemySpawn _asbp_game_mode)) 0))
        (CallFunction|SpawnAttackEnemy)))
    (:then_1
      (if (and (> (Variables|/Game/MiscBlueprints/BP_GameMode.BP_GameMode_C|GetNumSpeedEnemiesToSpawn (stale Custom|Round7EnemySpawn _asbp_game_mode)) 0) (> (Variables|Default|GetRound8SpeedEnemiesToSpawn) 0))
        (CallFunction|SpawnSpeedEnemy)))))

(event Custom|Round6EnemySpawn
  ;[0.1094 0.1094 0.1094] Spawning Enemies in Round 6
  (Utilities|FlowControl|Sequence
    (:then_0
      (if (and (> (Variables|Default|GetRound6AttackEnemiesToSpawn) 0) (> (Variables|/Game/MiscBlueprints/BP_GameMode.BP_GameMode_C|GetNumAttackEnemiesToSpawn (stale Custom|Round4EnemySpawn _asbp_game_mode)) 0))
        (CallFunction|SpawnAttackEnemy)))
    (:then_1
      (if (and (> (Variables|/Game/MiscBlueprints/BP_GameMode.BP_GameMode_C|GetNumSpeedEnemiesToSpawn (stale Custom|Round4EnemySpawn _asbp_game_mode)) 0) (> (Variables|Default|GetRound6SpeedEnemiesToSpawn) 0))
        (CallFunction|SpawnSpeedEnemy)))))

(event Custom|Round2EnemySpawn
  ;[0.1094 0.1094 0.1094] Spawning Enemies in Round 2
  (Utilities|FlowControl|Sequence
    (:then_0
      (if (and (> (Variables|Default|GetRound2AttackEnemiesToSpawn) 0) (> (Variables|/Game/MiscBlueprints/BP_GameMode.BP_GameMode_C|GetNumAttackEnemiesToSpawn (stale Custom|Round1EnemySpawn _asbp_game_mode)) 0))
        (CallFunction|SpawnAttackEnemy)))
    (:then_1
      (if (and (> (Variables|/Game/MiscBlueprints/BP_GameMode.BP_GameMode_C|GetNumSpeedEnemiesToSpawn (stale Custom|Round1EnemySpawn _asbp_game_mode)) 0) (> (Variables|Default|GetRound2SpeedEnemiesToSpawn) 0))
        (CallFunction|SpawnSpeedEnemy)))))

(event Custom|Round3EnemySpawn
  ;[0.1094 0.1094 0.1094] Spawning Enemies in Round 3
  (Utilities|FlowControl|Sequence
    (:then_0
      (if (and (> (Variables|Default|GetRound3AttackEnemiesToSpawn) 0) (> (Variables|/Game/MiscBlueprints/BP_GameMode.BP_GameMode_C|GetNumAttackEnemiesToSpawn (stale Custom|Round1EnemySpawn _asbp_game_mode)) 0))
        (CallFunction|SpawnAttackEnemy)))
    (:then_1
      (if (and (> (Variables|/Game/MiscBlueprints/BP_GameMode.BP_GameMode_C|GetNumSpeedEnemiesToSpawn (stale Custom|Round1EnemySpawn _asbp_game_mode)) 0) (> (Variables|Default|GetRound3SpeedEnemiesToSpawn) 0))
        (CallFunction|SpawnSpeedEnemy)))))

(event EventTick
  (params (DeltaSeconds :type Float%20%28single-precision%29))
  (CallFunction|InitializeRound)
  (bind _asbp_game_mode (Utilities|Casting|CastToBP_GameMode (Game|GetGameMode)))
  ;[0.1094 0.1094 0.1094] If player is in round spawn enemies
  (if (Variables|/Game/MiscBlueprints/BP_GameMode.BP_GameMode_C|GetInRound _asbp_game_mode)
    (if (Variables|Default|GetHasGlobalDelayHappened)
      _
      (else
        (Utilities|FlowControl|Delay (Variables|Default|GetGlobalSpawnDelay)) ; Spawn delay on spawner if you wanted to \nsay stagger certain lanes
        (Variables|Default|SetHasGlobalDelayHappened true)))
    ;[0.1094 0.1094 0.1094] Spawn enemies based on round
    (Utilities|FlowControl|Sequence
      (:then_0
        (if (== (Variables|/Game/MiscBlueprints/BP_GameMode.BP_GameMode_C|GetCurrentRound _asbp_game_mode) 1)
          (CallFunction|Round1EnemySpawn)))
      (:then_1
        (if (== (Variables|/Game/MiscBlueprints/BP_GameMode.BP_GameMode_C|GetCurrentRound _asbp_game_mode) 2)
          (CallFunction|Round2EnemySpawn)))
      (:then_2
        (if (== (Variables|/Game/MiscBlueprints/BP_GameMode.BP_GameMode_C|GetCurrentRound _asbp_game_mode) 3)
          (CallFunction|Round3EnemySpawn)))
      (:then_3
        (if (== (Variables|/Game/MiscBlueprints/BP_GameMode.BP_GameMode_C|GetCurrentRound _asbp_game_mode) 4)
          (CallFunction|Round4EnemySpawn)))
      (:then_4
        (if (== (Variables|/Game/MiscBlueprints/BP_GameMode.BP_GameMode_C|GetCurrentRound _asbp_game_mode) 5)
          (CallFunction|Round5EnemySpawn)))
      (:then_5
        (if (== (Variables|/Game/MiscBlueprints/BP_GameMode.BP_GameMode_C|GetCurrentRound _asbp_game_mode) 6)
          (CallFunction|Round6EnemySpawn)))
      (:then_6
        (if (== (Variables|/Game/MiscBlueprints/BP_GameMode.BP_GameMode_C|GetCurrentRound _asbp_game_mode) 7)
          (CallFunction|Round7EnemySpawn)))
      (:then_7
        (if (== (Variables|/Game/MiscBlueprints/BP_GameMode.BP_GameMode_C|GetCurrentRound _asbp_game_mode) 8)
          (CallFunction|Round8EnemySpawn))))
    (else
      (CallFunction|RoundComplete))))

(fn ConstructionScript)