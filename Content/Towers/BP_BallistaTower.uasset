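; Ballista tower for a tower defense game that tracks enemies inside its Sigh overlap component and shoots arrows at them, with a set sell price.
; Each tick it picks the closest overlapping enemy, intending to favor flying ones, and rotates the whole actor toward it.
; When the cooldown expires, it spawns BP_Arrow above the ballista along its reversed forward vector, plays a sound and briefly raises the Fired flag.
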(event EventBeginPlay
  (Variables|Default|SetSellPrice 200))

(event Collision|EventActorBeginOverlap
  (params (OtherActor :type Actor%20Object%20Reference)))

(event EventTick
  (params (DeltaSeconds :type Float%20%28single-precision%29))
  ;[1 1 1] count down fire timer
  (Variables|Default|SetFireCooldown (- (Variables|Default|GetFireCooldown) DeltaSeconds))
  (bind _closest (CallFunction|FindClosestEnemy))
  (Utilities|IsValid _closest
    (:Is%20Valid
      (CallFunction|AimatEnemy)
      (if (<= (Variables|Default|GetFireCooldown) 0.0)
        (CallFunction|ShootatEnemy)
        (Utilities|FlowControl|Delay 0.2)
        (Variables|Default|SetFired false)))))

(fn ConstructionScript)

(fn AimatEnemy
  (Transformation|SetActorRotation (Math|Rotator|FindLookatRotation (Transformation|GetActorLocation) (Transformation|GetActorLocation (Variables|Default|GetTargetEnemy)))))

(fn FindClosestEnemy
  (bind _self self)
  (bind _sigh (Variables|Default|GetSigh))
  (bind _overlappingactors (Collision|GetOverlappingActors _sigh "/Game/Enemies/BP_ParentEnemy.BP_ParentEnemy_C" :!class /Script/Engine.PrimitiveComponent))
  (Variables|Default|SetTargetEnemy (Utilities|Array|Get(acopy) _overlappingactors))
  (for (_array_element _array_index) _overlappingactors
    (if (!= _array_index 0)
      ;[1 1 1] prioritise flying enemies
      (if (== _array_element "/Game/Enemies/BP_FlyingEnemy.BP_FlyingEnemy")
        (Variables|Default|SetTargetEnemy _array_element :!label _label)
        (elif (<= (Transformation|GetDistanceTo _array_element _self) (Transformation|GetDistanceTo (Variables|Default|GetTargetEnemy) _self))
          (goto _label)))))
  (return (Variables|Default|GetTargetEnemy)))

(fn ShootatEnemy
  (bind _ballista (Variables|Default|GetBallista))
  (bind _returnvalue (Transformation|GetWorldTransform _ballista))
  (Game|SpawnActorfromClass "/Game/Towers/BP_Arrow.BP_Arrow_C" (Math|Transform|MakeTransform (Math|Vector|MakeVector (.x (.location _returnvalue)) (.y (.location _returnvalue)) (+ (.z (.location _returnvalue)) 1e+02)) (Math|Conversions|RotationFromXVector (* (Math|Vector|GetForwardVector (.rotation _returnvalue)) -1.0)) (.scale _returnvalue)) "Undefined" "MultiplyWithRoot" 0 0)
  (Variables|Default|SetFireCooldown 3.0)
  (Audio|PlaySoundatLocation "/Game/Sound/BallistaShoot.BallistaShoot" (Transformation|GetWorldLocation (Variables|Default|GetBallista)) "0, 0, 0" 1.0 1.0 0.0 0 0 0 0)
  (Variables|Default|SetFired true))