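; Tower that slows enemies inside its sphere trigger.
; On overlap it casts to BP_Enemy or BP_SpeedEnemy, sets a type-specific reduced walk speed and increments an in-range count.
; Leaving the sphere sets a hard-coded normal speed for that type and decrements the count.
; Tick uses the count to pause or unpause Freeze and activates SlowEffect while enemies are present, without ever deactivating it here.
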(event OnComponentBeginOverlap(Sphere)
  (params (OverlappedComponent :type Primitive%20Component%20Object%20Reference) (OtherActor :type Actor%20Object%20Reference) (OtherComp :type Primitive%20Component%20Object%20Reference) (OtherBodyIndex :type Integer) (bFromSweep :type Boolean) (SweepResult :type Hit%20Result%20Structure%20%28by%20ref%29))
  (bind _asbp_enemy (Utilities|Casting|CastToBP_Enemy OtherActor)
    (:then
      (Variables|/Script/Engine.CharacterMovementComponent|SetMaxWalkSpeed (Variables|/Script/Engine.Character|GetCharacterMovement _asbp_enemy) 25.0)
      (Variables|Default|SetenemiesInRange (+ (Variables|Default|GetenemiesInRange) 1)))
    (:CastFailed
      (bind _asbp_speed_enemy (Utilities|Casting|CastToBP_SpeedEnemy OtherActor))
      (Variables|/Script/Engine.CharacterMovementComponent|SetMaxWalkSpeed (Variables|/Script/Engine.Character|GetCharacterMovement _asbp_speed_enemy) 5e+01)
      (Variables|Default|SetenemiesInRange (+ (Variables|Default|GetenemiesInRange) 1)))))

(event OnComponentEndOverlap(Sphere)
  (params (OverlappedComponent :type Primitive%20Component%20Object%20Reference) (OtherActor :type Actor%20Object%20Reference) (OtherComp :type Primitive%20Component%20Object%20Reference) (OtherBodyIndex :type Integer))
  (bind _asbp_enemy (Utilities|Casting|CastToBP_Enemy OtherActor)
    (:then
      (Variables|/Script/Engine.CharacterMovementComponent|SetMaxWalkSpeed (Variables|/Script/Engine.Character|GetCharacterMovement _asbp_enemy) 1e+02)
      (Variables|Default|SetenemiesInRange (- (Variables|Default|GetenemiesInRange) 1)))
    (:CastFailed
      (bind _asbp_speed_enemy (Utilities|Casting|CastToBP_SpeedEnemy OtherActor))
      (Variables|/Script/Engine.CharacterMovementComponent|SetMaxWalkSpeed (Variables|/Script/Engine.Character|GetCharacterMovement _asbp_speed_enemy) 3e+02)
      (Variables|Default|SetenemiesInRange (- (Variables|Default|GetenemiesInRange) 1)))))

(event EventBeginPlay)

(event Collision|EventActorBeginOverlap
  (params (OtherActor :type Actor%20Object%20Reference)))

(event EventTick
  (params (DeltaSeconds :type Float%20%28single-precision%29))
  (bind _freeze (Variables|Default|GetFreeze))
  (if (> (Variables|Default|GetenemiesInRange) 0)
    (Class|AudioComponent|SetPaused _freeze false)
    (Components|Activation|Activate (Variables|Default|Getslow%20effect) false)
    (else
      (Class|AudioComponent|SetPaused _freeze true))))

(fn ConstructionScript)