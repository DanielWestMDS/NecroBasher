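; BP_LaserTower is a tower that periodically fires a laser, killing enemies its hitbox touches.
; Tick cycles with latent Delays: wait the fire interval, activate the beam VFX, wait for it to charge, then set LaserFired briefly.
; That flag teleports the hitbox between raised (on) and lowered (off) positions rather than toggling collision.
; Begin-overlap sets the Health of BP_Enemy or BP_SpeedEnemy to zero.
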(event OnComponentBeginOverlap(Hitbox)
  (params (OverlappedComponent :type Primitive%20Component%20Object%20Reference) (OtherActor :type Actor%20Object%20Reference) (OtherComp :type Primitive%20Component%20Object%20Reference) (OtherBodyIndex :type Integer) (bFromSweep :type Boolean) (SweepResult :type Hit%20Result%20Structure%20%28by%20ref%29))
  (bind _asbp_enemy (Utilities|Casting|CastToBP_Enemy OtherActor)
    (:then
      (Variables|/Game/Enemies/BP_Enemy.BP_Enemy_C|SetHealth _asbp_enemy 0.0))
    (:CastFailed
      (bind _asbp_speed_enemy (Utilities|Casting|CastToBP_SpeedEnemy OtherActor))
      (Variables|/Game/Enemies/BP_SpeedEnemy.BP_SpeedEnemy_C|SetHealth _asbp_speed_enemy 0.0))))

(event EventBeginPlay)

(event Collision|EventActorBeginOverlap
  (params (OtherActor :type Actor%20Object%20Reference)))

(event EventTick
  (params (DeltaSeconds :type Float%20%28single-precision%29))
  (if (Variables|Default|GetLaserFired)
    ;[1 1 1] laser on
    (Transformation|SetRelativeLocation (Variables|Default|GetHitbox) "0.000000,0.000000,170.000000" false false)
    (Utilities|FlowControl|Delay 0.3)
    (Variables|Default|SetLaserFired false)
    (else
      ;[1 1 1] laser off
      (Transformation|SetRelativeLocation (Variables|Default|GetHitbox) "0.000000,0.000000,-170.000000" false false)
      (Utilities|FlowControl|Delay (Variables|Default|Getfireinterval))
      (Components|Activation|Activate (Variables|Default|GetVFX_Beam) true)
      (Utilities|FlowControl|Delay 1.55)
      (Variables|Default|SetLaserFired true))))

(fn ConstructionScript)