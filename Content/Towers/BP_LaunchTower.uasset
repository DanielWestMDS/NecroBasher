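; Launch trap tower that knocks BP_Enemy and BP_SpeedEnemy characters backward, with a cooldown.
; An enemy entering TriggerRadius sets LaunchTriggered and scales up EffectRadius, using the resulting overlap events as an area hit.
; Each overlapped enemy is flagged, stopped and launched horizontally against its facing, then EffectRadius shrinks and a sound plays.
; Tick clears LaunchTriggered through a fixed Delay, re-arming the trap.
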(event OnComponentBeginOverlap(TriggerRadius)
  (params (OverlappedComponent :type Primitive%20Component%20Object%20Reference) (OtherActor :type Actor%20Object%20Reference) (OtherComp :type Primitive%20Component%20Object%20Reference) (OtherBodyIndex :type Integer) (bFromSweep :type Boolean) (SweepResult :type Hit%20Result%20Structure%20%28by%20ref%29))
  (Utilities|Casting|CastToBP_Enemy OtherActor
    (:then
      _)
    (:CastFailed
      (Utilities|Casting|CastToBP_SpeedEnemy OtherActor)))
  (if (not (Variables|Default|GetbLaunchTriggered))
    (Variables|Default|SetbLaunchTriggered true)
    (Transformation|SetWorldScale3D (Variables|Default|GetEffectRadius) "9.500000,9.500000,9.500000")))

(event OnComponentBeginOverlap(EffectRadius)
  (params (OverlappedComponent :type Primitive%20Component%20Object%20Reference) (OtherActor :type Actor%20Object%20Reference) (OtherComp :type Primitive%20Component%20Object%20Reference) (OtherBodyIndex :type Integer) (bFromSweep :type Boolean) (SweepResult :type Hit%20Result%20Structure%20%28by%20ref%29))
  (if (Variables|Default|GetbLaunchTriggered)
    (bind _asbp_enemy (Utilities|Casting|CastToBP_Enemy OtherActor)
      (:then
        (Variables|/Game/Enemies/BP_Enemy.BP_Enemy_C|SetisBeingLaunched _asbp_enemy true)
        (Class|NavMovementComponent|StopActiveMovement (Variables|/Script/Engine.Character|GetCharacterMovement _asbp_enemy))
        (Character|LaunchCharacter _asbp_enemy (* (Math|Vector|GetForwardVector (Transformation|GetActorRotation _asbp_enemy)) "-10000.000000,-10000.000000,0.000000") true false))
      (:CastFailed
        (bind _asbp_speed_enemy (Utilities|Casting|CastToBP_SpeedEnemy OtherActor))
        (Variables|/Game/Enemies/BP_SpeedEnemy.BP_SpeedEnemy_C|SetisBeingLaunched _asbp_speed_enemy true)
        (Class|NavMovementComponent|StopActiveMovement (Variables|/Script/Engine.Character|GetCharacterMovement _asbp_speed_enemy))
        (Character|LaunchCharacter _asbp_speed_enemy (* (Math|Vector|GetForwardVector (Transformation|GetActorRotation _asbp_speed_enemy)) "-10000.000000,-10000.000000,0.000000") true false)))
    (Transformation|SetWorldScale3D (Variables|Default|GetEffectRadius) "0.100000,0.100000,0.100000")
    (Audio|PlaySoundatLocation "/Game/Sound/launchTrap.launchTrap" (Transformation|GetWorldLocation (Variables|Default|GetDefaultSceneRoot)) "0, 0, 0" 1.0 1.0 0.0 0 0 0 0)))

(event EventBeginPlay)

(event Collision|EventActorBeginOverlap
  (params (OtherActor :type Actor%20Object%20Reference)))

(event EventTick
  (params (DeltaSeconds :type Float%20%28single-precision%29))
  (if (Variables|Default|GetbLaunchTriggered)
    (Utilities|FlowControl|Delay 15.0)
    (Variables|Default|SetbLaunchTriggered false)))

(fn ConstructionScript)