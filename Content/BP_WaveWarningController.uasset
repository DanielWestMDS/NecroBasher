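; Wave warning controller that shows and hides spline warning actors for three lanes, driven by Lane1–3Warning flags on BP_GameMode.
; Everything starts hidden; each Tick shows the flagged lane's spline pair through SetArrayVisible.
; A single shared LaneTimer runs during rounds, triggering blinking after half of DisappearTimer and clearing the warning at its end.
; The blink step toggles splines 0 and 1 for every lane, not each lane's own pair.
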(event Custom|SetWarningVisible
  (bind _gamemodereference (Variables|Default|GetGamemodeReference))
  (Utilities|FlowControl|Sequence
    (:then_0
      (if (Variables|/Game/MiscBlueprints/BP_GameMode.BP_GameMode_C|GetLane1Warning _gamemodereference)
        (CallFunction|SetArrayVisible 0 true)
        (CallFunction|SetArrayVisible 1 true)
        (if (> (Variables|Default|GetLaneTimer) (/ (Variables|Default|GetDisappearTimer) 2.0))
          (if (== (Math|Float|Round (Math|Float|%(Float) (* (Variables|Default|GetLaneTimer) 2.0) 2.0)) 1)
            (CallFunction|SetArrayVisible 0 true)
            (CallFunction|SetArrayVisible 1 true)
            (else
              (CallFunction|SetArrayVisible 0 false)
              (CallFunction|SetArrayVisible 1 false)))
          (if (> (Variables|Default|GetLaneTimer) (Variables|Default|GetDisappearTimer))
            (Variables|/Game/MiscBlueprints/BP_GameMode.BP_GameMode_C|SetLane1Warning (Variables|Default|GetGamemodeReference) false)
            (CallFunction|SetArrayVisible 0 false)
            (CallFunction|SetArrayVisible 1 false)
            (Variables|Default|SetLaneTimer 0.0)))))
    (:then_1
      (if (Variables|/Game/MiscBlueprints/BP_GameMode.BP_GameMode_C|GetLane2Warning _gamemodereference)
        (CallFunction|SetArrayVisible 3 true)
        (CallFunction|SetArrayVisible 4 true)
        (if (> (Variables|Default|GetLaneTimer) (/ (Variables|Default|GetDisappearTimer) 2.0))
          (if (== (Math|Float|Round (Math|Float|%(Float) (* (Variables|Default|GetLaneTimer) 2.0) 2.0)) 1)
            (CallFunction|SetArrayVisible 0 true)
            (CallFunction|SetArrayVisible 1 true)
            (else
              (CallFunction|SetArrayVisible 0 false)
              (CallFunction|SetArrayVisible 1 false)))
          (if (> (Variables|Default|GetLaneTimer) (Variables|Default|GetDisappearTimer))
            (Variables|/Game/MiscBlueprints/BP_GameMode.BP_GameMode_C|SetLane2Warning (Variables|Default|GetGamemodeReference) false)
            (CallFunction|SetArrayVisible 3 false)
            (CallFunction|SetArrayVisible 4 false)
            (Variables|Default|SetLaneTimer 0.0)))))
    (:then_2
      (if (Variables|/Game/MiscBlueprints/BP_GameMode.BP_GameMode_C|GetLane3Warning _gamemodereference)
        (CallFunction|SetArrayVisible 5 true)
        (CallFunction|SetArrayVisible 6 true)
        (if (> (Variables|Default|GetLaneTimer) (/ (Variables|Default|GetDisappearTimer) 2.0))
          (if (== (Math|Float|Round (Math|Float|%(Float) (* (Variables|Default|GetLaneTimer) 2.0) 2.0)) 1)
            (CallFunction|SetArrayVisible 0 true)
            (CallFunction|SetArrayVisible 1 true)
            (else
              (CallFunction|SetArrayVisible 0 false)
              (CallFunction|SetArrayVisible 1 false)))
          (if (> (Variables|Default|GetLaneTimer) (Variables|Default|GetDisappearTimer))
            (Variables|/Game/MiscBlueprints/BP_GameMode.BP_GameMode_C|SetLane3Warning (Variables|Default|GetGamemodeReference) false)
            (CallFunction|SetArrayVisible 5 false)
            (CallFunction|SetArrayVisible 6 false)
            (Variables|Default|SetLaneTimer 0.0)))))))

(event EventBeginPlay
  (bind _asbp_game_mode (Utilities|Casting|CastToBP_GameMode (Game|GetGameMode)))
  (Variables|Default|SetGamemodeReference _asbp_game_mode)
  (for _array_element (Variables|Default|GetWaveWarningSplineArray)
    (for _array_element_2 (Variables|/Game/Enemies/Splines/BP_WaveWarningError.BP_WaveWarningError_C|GetActor _array_element)
      (Rendering|SetVisibility (Variables|/Script/Engine.Actor|GetRootComponent _array_element_2) false false))))

(event EventTick
  (params (DeltaSeconds :type Float%20%28single-precision%29))
  (CallFunction|SetWarningVisible)
  (if (Variables|/Game/MiscBlueprints/BP_GameMode.BP_GameMode_C|GetInRound (Variables|Default|GetGamemodeReference))
    (Variables|Default|SetLaneTimer (+ (Utilities|Time|GetWorldDeltaSeconds) (Variables|Default|GetLaneTimer)))
    (else
      (Variables|Default|SetLaneTimer 0.0))))

(fn ConstructionScript)

(fn SetArrayVisible
  (params (Spline :type Integer) (IsVisible :type Boolean))
  (for _array_element (Variables|/Game/Enemies/Splines/BP_WaveWarningError.BP_WaveWarningError_C|GetActor (Utilities|Array|Get(acopy) (Variables|Default|GetWaveWarningSplineArray) Spline))
    (Rendering|SetVisibility (Variables|/Script/Engine.Actor|GetRootComponent _array_element) IsVisible false)))